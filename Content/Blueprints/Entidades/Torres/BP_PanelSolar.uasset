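; BP_PanelSolar is a solar panel tower entity that handles its production and death animations.
; BeginPlay binds two animation components to the Placas component, giving AnimPaneles a red material for the producing state.
; RealizarAnimacion uses an index to start death on a timer, or produce and stop-producing animations via CrearAnimacionSinTimer, dispatched by function name.
; DestruirAnimaciones clears both components' timers and stops the panel audio.
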(event EventBeginPlay
  (Default|Inicializar (Variables|Default|GetAnim%20Paneles) (Variables|Default|GetPlacas) "/Game/Assets/Materiales/MisMateriales/M_Rojo.M_Rojo" 2)
  (Default|Inicializar (Variables|Default|GetAnimar%20Muerte) (Variables|Default|GetPlacas)))

(event EventDestruirAnimaciones
  (bind _anim_paneles (Variables|Default|GetAnim%20Paneles))
  (Default|BorrarTimer _anim_paneles)
  (Default|BorrarTimer (Variables|Default|GetAnimar%20Muerte))
  (Default|PararAudio _anim_paneles))

(event EventRealizarAnimacion
  (params (Animacion :type Integer))
  (CallFunction|ElegirAnimacion Animacion))

(fn ConstructionScript)

(fn ElegirAnimacion
  (params (Seleccion :type Integer))
  (bind _animar_muerte (Variables|Default|GetAnimar%20Muerte))
  (bind _anim_paneles (Variables|Default|GetAnim%20Paneles))
  (bind _deltatime (Variables|/Game/Blueprints/Utilidad_Animacion/BP_Anim_TimerBlueprint.BP_Anim_TimerBlueprint_C|GetDeltaTime _anim_paneles))
  (switch int Seleccion
    (:0
      (Default|CrearTimer _animar_muerte "Animar Muerte" _animar_muerte))
    (:1
      (Default|CrearAnimacionSinTimer _anim_paneles "Animar Desproducir" _anim_paneles _deltatime))
    (:2
      (Default|CrearAnimacionSinTimer _anim_paneles "Animar Producir" _anim_paneles _deltatime))))