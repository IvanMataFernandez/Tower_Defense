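; BP_Mina is a mine in the tower entities that drives its visual animations.
; On BeginPlay it initializes three animation components for ready, explosion countdown and death, using the tip and base meshes with yellow and red flash materials.
; An animation event maps an ID to the matching component, which starts its animation on a timer, and a cleanup event clears all three timers.
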(event EventBeginPlay
  (Default|Inicializar (Variables|Default|GetAnimar%20Preparado) (Variables|Default|GetPunta) 0 "/Game/Assets/Materiales/MisMateriales/M_Amarillo.M_Amarillo")
  (Default|Inicializar (Variables|Default|GetAnimar%20Explosion) (Variables|Default|GetPunta) 0 "/Game/Assets/Materiales/MisMateriales/M_Rojo.M_Rojo" 0.8 false)
  (Default|Inicializar (Variables|Default|GetAnimar%20Muerte) (Variables|Default|GetPunta) (Variables|Default|GetCuerpoBase)))

(event EventDestruirAnimaciones
  (Default|BorrarTimer (Variables|Default|GetAnimar%20Preparado))
  (Default|BorrarTimer (Variables|Default|GetAnimar%20Explosion))
  (Default|BorrarTimer (Variables|Default|GetAnimar%20Muerte)))

(event EventRealizarAnimacion
  (params (Animacion :type Integer))
  (CallFunction|ElegirAnimacion Animacion))

(fn ConstructionScript)

(fn ElegirAnimacion
  (params (Id :type Integer))
  (switch int Id
    (:0
      (Default|CrearTimer (Variables|Default|GetAnimar%20Muerte) "Animar Muerte"))
    (:1
      (Default|CrearTimer (Variables|Default|GetAnimar%20Explosion) "Animar Countdown Explosion"))
    (:2
      (Default|CrearTimer (Variables|Default|GetAnimar%20Preparado) "Preparado"))))