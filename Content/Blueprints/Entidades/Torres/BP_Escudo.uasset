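; Shield tower Blueprint that drives its rotation, deterioration and death animations.
; BeginPlay sets up animation helpers: a rotator for each of the three shield parts, a deterioration helper fed by those rotators, and a death helper using the third rotator and body.
; RealizarAnimacion dispatches an ID to start timer-driven rotation or death, trigger timerless deterioration, or stop the third rotator.
; DestruirAnimaciones clears the rotation and death timers.
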(event EventBeginPlay
  (Default|Inicializar (Variables|Default|GetAnim%20Rotar%20Escudo%201) (Variables|Default|GetEscudo1) 9e+01)
  (Default|Inicializar (Variables|Default|GetAnim%20Rotar%20Escudo%202) (Variables|Default|GetEscudo2) 9e+01)
  (Default|Inicializar (Variables|Default|GetAnim%20Rotar%20Escudo%203) (Variables|Default|GetEscudo3) 9e+01)
  (Default|Inicializar (Variables|Default|GetAnim%20Deterioro) (Variables|Default|GetAnim%20Rotar%20Escudo%201) (Variables|Default|GetAnim%20Rotar%20Escudo%202) (Variables|Default|GetAnim%20Rotar%20Escudo%203))
  (Default|Inicializar (Variables|Default|GetAnimar%20Muerte) (Variables|Default|GetAnim%20Rotar%20Escudo%203) (Variables|Default|GetCuerpoEscudo)))

(event EventDestruirAnimaciones
  (Default|BorrarTimer (Variables|Default|GetAnim%20Rotar%20Escudo%201))
  (Default|BorrarTimer (Variables|Default|GetAnim%20Rotar%20Escudo%202))
  (Default|BorrarTimer (Variables|Default|GetAnim%20Rotar%20Escudo%203))
  (Default|BorrarTimer (Variables|Default|GetAnimar%20Muerte)))

(event EventRealizarAnimacion
  (params (Animacion :type Integer))
  (CallFunction|ElegirAnimacion Animacion))

(fn ConstructionScript)

(fn ElegirAnimacion
  (params (Id :type Integer))
  (switch int Id
    (:-2
      (Default|CrearAnimacionSinTimer (Variables|Default|GetAnim%20Deterioro) "Deteriorar" 0.01 :!label _label))
    (:-1
      (goto _label))
    (:0
      (Default|CrearTimer (Variables|Default|GetAnimar%20Muerte) "Animar Muerte"))
    (:1
      (Default|CrearTimer (Variables|Default|GetAnim%20Rotar%20Escudo%201) "Rotar Componente")
      (Default|CrearTimer (Variables|Default|GetAnim%20Rotar%20Escudo%202) "Rotar Componente")
      (Default|CrearTimer (Variables|Default|GetAnim%20Rotar%20Escudo%203) "Rotar Componente"))
    (:2
      (Default|BorrarTimer (Variables|Default|GetAnim%20Rotar%20Escudo%203)))))