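; BP_PanelSolarDoble is a double solar panel building among the tower entities, handling its production and death animations.
; On BeginPlay it binds the AnimPaneles and AnimarMuerte helpers to the Placas component, giving AnimPaneles a red producing material.
; RealizarAnimacion selects death, stop-producing or producing animations, started by function name through those helpers.
; DestruirAnimaciones clears both helpers' timers and stops the panel audio.
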(event EventBeginPlay
  (bind _placas (Variables|Default|GetPlacas))
  (Default|Inicializar (Variables|Default|GetAnim%20Paneles) _placas "/Game/Assets/Materiales/MisMateriales/M_Rojo.M_Rojo" 1)
  (Default|Inicializar (Variables|Default|GetAnimar%20Muerte) _placas))

(event EventDestruirAnimaciones
  (bind _anim_paneles (Variables|Default|GetAnim%20Paneles))
  (Default|BorrarTimer _anim_paneles)
  (Default|BorrarTimer (Variables|Default|GetAnimar%20Muerte))
  (Default|PararAudio _anim_paneles))

(event EventRealizarAnimacion
  (params (Animacion :type Integer))
  (CallFunction|ElegirAnimacion Animacion))

(fn ConstructionScript)

(fn ElegirAnimacion
  (params (Seleccion :type Integer))
  (bind _anim_paneles (Variables|Default|GetAnim%20Paneles))
  (switch int Seleccion
    (:0
      (Default|CrearTimer (Variables|Default|GetAnimar%20Muerte) "Animar Muerte"))
    (:1
      (Default|CrearAnimacionSinTimer _anim_paneles "Animar Desproducir" 0.01))
    (:2
      (Default|CrearAnimacionSinTimer _anim_paneles "Animar Producir" 0.01))))