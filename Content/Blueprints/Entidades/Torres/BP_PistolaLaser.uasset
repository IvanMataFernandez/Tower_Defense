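; BP_PistolaLaser is the laser pistol tower, and this Blueprint handles its animations.
; BeginPlay initializes two helpers on the Pistola component: AnimCaraLaser, given red and black materials, and AnimarMuerte for death.
; RealizarAnimacion passes an animation ID to ElegirAnimacion, which triggers death, un-aim, aim or shot animations by function name, mostly on timers.
; DestruirAnimaciones clears both helpers' timers.
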(event EventBeginPlay
  (bind _pistola (Variables|Default|GetPistola))
  (Default|Inicializar (Variables|Default|GetAnim%20Cara%20Laser) _pistola 1 "/Game/Assets/Materiales/MisMateriales/M_Rojo.M_Rojo" "/Game/Assets/Materiales/MisMateriales/M_Negro.M_Negro")
  (Default|Inicializar (Variables|Default|GetAnimar%20Muerte) _pistola))

(event EventDestruirAnimaciones
  (Default|BorrarTimer (Variables|Default|GetAnim%20Cara%20Laser))
  (Default|BorrarTimer (Variables|Default|GetAnimar%20Muerte)))

(event EventRealizarAnimacion
  (params (Animacion :type Integer))
  (CallFunction|ElegirAnimacion Animacion))

(fn ConstructionScript)

(fn ElegirAnimacion
  (params (Id :type Integer))
  (bind _anim_cara_laser (Variables|Default|GetAnim%20Cara%20Laser))
  (switch int Id
    (:0
      (Default|CrearTimer (Variables|Default|GetAnimar%20Muerte) "Animar Muerte"))
    (:1
      (Default|CrearTimer _anim_cara_laser "Desapuntar"))
    (:2
      (Default|CrearTimer _anim_cara_laser "Apuntar"))
    (:3
      (Default|CrearAnimacionSinTimer _anim_cara_laser "Disparo" 0.0001))))