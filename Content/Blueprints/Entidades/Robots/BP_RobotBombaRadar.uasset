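; Robot entity Blueprint for a bomb radar robot, handling its procedural animations: wheel movement, laser face firing, detonation countdown flash and three spinning propellers.
; BeginPlay initializes one animation component per effect with its target mesh, materials and speeds.
; RealizarAnimacion passes an ID to ElegirAnimacion, which starts named timer-driven animations, fires the timerless shot, or stops the wheels.
; DestruirAnimaciones clears every animation timer.
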(event EventBeginPlay
  (Default|Inicializar (Variables|Default|GetAnim%20Cara%20Laser) (Variables|Default|GetMeshDisparador) 0 "/Game/Assets/Materiales/MisMateriales/M_Rojo.M_Rojo")
  (Default|Inicializar (Variables|Default|GetAnim%20Bomba%20Detonar) (Variables|Default|GetCuerpoBase) 2 "/Game/Assets/Materiales/MisMateriales/M_Rojo.M_Rojo" 1.8)
  (Default|Inicializar (Variables|Default|GetAnim%20Mover%20Ruedas) (Variables|Default|GetMeshDesplazador) (Variables|Default|GetVelocidadBase) 59.0)
  (Default|Inicializar (Variables|Default|GetAnim%20Rotar%20Helice%201) (Variables|Default|GetHelice%201) 3.6e+02)
  (Default|Inicializar (Variables|Default|GetAnim%20Rotar%20Helice%202) (Variables|Default|GetHelice%202) 3.6e+02)
  (Default|Inicializar (Variables|Default|GetAnim%20Rotar%20Helice%203) (Variables|Default|GetHelice%203) 3.6e+02))

(event EventDestruirAnimaciones
  (Default|BorrarTimer (Variables|Default|GetAnim%20Cara%20Laser))
  (Default|BorrarTimer (Variables|Default|GetAnim%20Bomba%20Detonar))
  (Default|BorrarTimer (Variables|Default|GetAnim%20Mover%20Ruedas))
  (Default|BorrarTimer (Variables|Default|GetAnim%20Rotar%20Helice%201))
  (Default|BorrarTimer (Variables|Default|GetAnim%20Rotar%20Helice%202))
  (Default|BorrarTimer (Variables|Default|GetAnim%20Rotar%20Helice%203)))

(event EventRealizarAnimacion
  (params (Animacion :type Integer))
  (CallFunction|ElegirAnimacion Animacion))

(fn ConstructionScript)

(fn ElegirAnimacion
  (params (Id :type Integer))
  (bind _anim_cara_laser (Variables|Default|GetAnim%20Cara%20Laser))
  (bind _anim_bomba_detonar (Variables|Default|GetAnim%20Bomba%20Detonar))
  (bind _anim_mover_ruedas (Variables|Default|GetAnim%20Mover%20Ruedas))
  (bind _anim_rotar_helice_1 (Variables|Default|GetAnim%20Rotar%20Helice%201))
  (bind _anim_rotar_helice_2 (Variables|Default|GetAnim%20Rotar%20Helice%202))
  (bind _anim_rotar_helice_3 (Variables|Default|GetAnim%20Rotar%20Helice%203))
  (switch int Id
    (:-1
      (Default|BorrarTimer _anim_mover_ruedas))
    (:1
      (Default|CrearTimer _anim_mover_ruedas "Rotar Rueda" _anim_mover_ruedas))
    (:2
      (Default|CrearAnimacionSinTimer _anim_cara_laser "Disparo" _anim_cara_laser 0.2))
    (:3
      (Default|CrearTimer _anim_bomba_detonar "Animar Countdown Explosion" _anim_bomba_detonar))
    (:4
      (Default|CrearTimer _anim_rotar_helice_1 "Rotar Componente" _anim_rotar_helice_1)
      (Default|CrearTimer _anim_rotar_helice_2 "Rotar Componente" _anim_rotar_helice_2)
      (Default|CrearTimer _anim_rotar_helice_3 "Rotar Componente" _anim_rotar_helice_3))))