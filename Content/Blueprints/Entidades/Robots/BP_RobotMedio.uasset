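; BP_RobotMedio is the medium robot entity, handling its visual animations through dedicated animation components.
; BeginPlay initializes the laser face, wheel rotation, death and deterioration components with their meshes, materials and movement parameters.
; RealizarAnimacion maps an integer ID to medium or heavy damage, death, wheel start/stop or firing, using either timers or timerless animations.
; DestruirAnimaciones clears the laser, death and wheel timers.
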(event EventBeginPlay
  (Default|Inicializar (Variables|Default|GetAnim%20Cara%20Laser) (Variables|Default|GetMeshDisparador) 0 "/Game/Assets/Materiales/MisMateriales/M_Rojo.M_Rojo")
  (Default|Inicializar (Variables|Default|GetAnim%20Mover%20Ruedas) (Variables|Default|GetMeshDesplazador) (Variables|Default|GetVelocidadBase) 59.0)
  (Default|Inicializar (Variables|Default|GetAnimar%20Muerte) (Variables|Default|GetPosicionBase))
  (Default|Inicializar (Variables|Default|GetAnim%20Deterioro) "/Game/Assets/Materiales/MisMateriales/M_AmarilloAlgoDañado.M_AmarilloAlgoDañado" "/Game/Assets/Materiales/MisMateriales/M_VerdeAlgoDañado.M_VerdeAlgoDañado" "/Game/Assets/Materiales/MisMateriales/M_AmarilloMuyDañado.M_AmarilloMuyDañado" "/Game/Assets/Materiales/MisMateriales/M_VerdeMuyDañado.M_VerdeMuyDañado" (Variables|Default|GetCuerpoBase)))

(event EventDestruirAnimaciones
  (Default|BorrarTimer (Variables|Default|GetAnim%20Cara%20Laser))
  (Default|BorrarTimer (Variables|Default|GetAnimar%20Muerte))
  (Default|BorrarTimer (Variables|Default|GetAnim%20Mover%20Ruedas)))

(event EventRealizarAnimacion
  (params (Animacion :type Integer))
  (CallFunction|ElegirAnimacion Animacion))

(fn ConstructionScript)

(fn ElegirAnimacion
  (params (Id :type Integer))
  (bind _anim_cara_laser (Variables|Default|GetAnim%20Cara%20Laser))
  (bind _anim_mover_ruedas (Variables|Default|GetAnim%20Mover%20Ruedas))
  (bind _animar_muerte (Variables|Default|GetAnimar%20Muerte))
  (bind _anim_deterioro (Variables|Default|GetAnim%20Deterioro))
  (switch int Id
    (:-2
      (Default|CrearAnimacionSinTimer _anim_deterioro "Deterioro Medio" _anim_deterioro 0.01))
    (:-1
      (Default|CrearAnimacionSinTimer _anim_deterioro "Deterioro Alto" _anim_deterioro 0.01))
    (:0
      (Default|CrearTimer _animar_muerte "Animar Muerte" _animar_muerte))
    (:1
      (Default|CrearTimer _anim_mover_ruedas "Rotar Rueda" _anim_mover_ruedas))
    (:2
      (Default|BorrarTimer (Variables|Default|GetAnim%20Mover%20Ruedas)))
    (:3
      (Default|CrearAnimacionSinTimer _anim_cara_laser "Disparo" _anim_cara_laser 0.2))))