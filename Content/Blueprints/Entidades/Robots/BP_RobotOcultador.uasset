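; Blueprint for the Ocultador robot, which drives its animations: rolling wheel halves, laser face shot, hiding and unhiding protectors, deterioration and death.
; BeginPlay initializes one animation helper per effect with the body, wheel and shooter meshes, plus materials for attack and damage.
; RealizarAnimacion maps an integer ID to timer-driven or timerless helper animations.
; DestruirAnimaciones clears only the laser face and wheel rotation timers.
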(event EventBeginPlay
  (bind _cuerpobase (Variables|Default|GetCuerpoBase))
  (bind _meshdesplazador (Variables|Default|GetMeshDesplazador))
  (bind _mesh_desplazador_2 (Variables|Default|GetMesh%20Desplazador%202))
  (Default|Inicializar (Variables|Default|GetAnim%20Cara%20Laser) (Variables|Default|GetMeshDisparador) 1 "/Game/Assets/Materiales/MisMateriales/M_Rojo.M_Rojo")
  (Default|Inicializar (Variables|Default|GetAnim%20Rotar%20Mitad1) (Variables|Default|GetMeshDesplazador) (Variables|Default|GetVelocidadBase) 142.0)
  (Default|Inicializar (Variables|Default|GetAnim%20Rotar%20Mitad2) (Variables|Default|GetMesh%20Desplazador%202) (Variables|Default|GetVelocidadBase) 142.0)
  (Default|Inicializar (Variables|Default|GetAnim%20Protectores) _cuerpobase _mesh_desplazador_2 _meshdesplazador)
  (Default|Inicializar (Variables|Default|GetAnim%20Deterioro) _cuerpobase _meshdesplazador _mesh_desplazador_2 "/Game/Assets/Materiales/MisMateriales/M_VerdeOscuroMuyDañado.M_VerdeOscuroMuyDañado" "/Game/Assets/Materiales/MaterialsBundle/Masters/M_Metal_Damaged.M_Metal_Damaged")
  (Default|Inicializar (Variables|Default|GetAnimar%20Muerte) (Variables|Default|GetCuerpoBase) (Variables|Default|GetMesh%20Desplazador%202) (Variables|Default|GetMeshDesplazador)))

(event EventDestruirAnimaciones
  (Default|BorrarTimer (Variables|Default|GetAnim%20Cara%20Laser))
  (Default|BorrarTimer (Variables|Default|GetAnim%20Rotar%20Mitad1))
  (Default|BorrarTimer (Variables|Default|GetAnim%20Rotar%20Mitad2)))

(event EventRealizarAnimacion
  (params (Animacion :type Integer))
  (CallFunction|ElegirAnimacion Animacion))

(fn ConstructionScript)

(fn ElegirAnimacion
  (params (Id :type Integer))
  (bind _anim_rotar_mitad1 (Variables|Default|GetAnim%20Rotar%20Mitad1))
  (bind _anim_rotar_mitad2 (Variables|Default|GetAnim%20Rotar%20Mitad2))
  (switch int Id
    (:-1
      (Default|CrearAnimacionSinTimer (Variables|Default|GetAnim%20Deterioro) "Deteriorar" 0.01))
    (:0
      (Default|CrearTimer (Variables|Default|GetAnimar%20Muerte) "Animar Muerte"))
    (:1
      (Default|CrearTimer _anim_rotar_mitad1 "Rotar Rueda")
      (Default|CrearTimer _anim_rotar_mitad2 "Rotar Rueda"))
    (:2
      (Default|BorrarTimer _anim_rotar_mitad1)
      (Default|BorrarTimer _anim_rotar_mitad2))
    (:3
      (Default|CrearAnimacionSinTimer (Variables|Default|GetAnim%20Cara%20Laser) "Disparo" 0.01))
    (:4
      (Default|CrearTimer (Variables|Default|GetAnim%20Protectores) "Desocultar"))
    (:5
      (Default|CrearTimer (Variables|Default|GetAnim%20Protectores) "Ocultar"))))