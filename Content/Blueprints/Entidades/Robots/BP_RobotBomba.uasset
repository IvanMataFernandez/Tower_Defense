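; BP_RobotBomba is a bomb robot entity Blueprint that drives the robot's wheel, laser-face attack and detonation animations.
; On BeginPlay it initializes three animation components on the shooter, body and locomotion meshes, using red materials for attack and flash effects.
; RealizarAnimacion maps an ID through ElegirAnimacion to a component and function name, then starts that component's timer.
; A negative ID clears the wheel timer.
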(event EventBeginPlay
  (Default|Inicializar (Variables|Default|GetAnim%20Cara%20Laser) (Variables|Default|GetMeshDisparador) 0 "/Game/Assets_Mios/Materiales/M_Rojo.M_Rojo")
  (Default|Inicializar (Variables|Default|GetAnim%20Bomba%20Detonar) (Variables|Default|GetCuerpoBase) 1 "/Game/Assets_Mios/Materiales/M_Rojo.M_Rojo")
  (Default|Inicializar (Variables|Default|GetAnim%20Mover%20Ruedas) (Variables|Default|GetMeshDesplazador) (Variables|Default|GetVelocidadBase) 59.0))

(event EventRealizarAnimacion
  (params (Animacion :type Integer))
  (if (>= Animacion 0)
    (bind (_funcion _anim_componente) (CallFunction|ElegirAnimacion Animacion))
    (Default|CrearTimer _anim_componente _funcion _anim_componente)
    (else
      (Default|BorrarTimer (Variables|Default|GetAnim%20Mover%20Ruedas)))))

(fn ConstructionScript)

(fn ElegirAnimacion
  (params (Id :type Integer))
  (switch int Id
    (:0
      (return "Rotar Rueda" (Variables|Default|GetAnim%20Mover%20Ruedas)))
    (:1
      (return "Disparo" (Variables|Default|GetAnim%20Cara%20Laser)))
    (:2
      (return "Animar Countdown Explosion" (Variables|Default|GetAnim%20Bomba%20Detonar)))))