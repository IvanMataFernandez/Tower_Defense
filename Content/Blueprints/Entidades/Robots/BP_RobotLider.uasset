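; BP_RobotLider is the leader robot, a child of a robot parent class that adds a rotating flag.
; BeginPlay passes red damaged materials for body and side to the inherited setup and binds a RotarBandera helper to the flag component.
; The animation selection override calls the parent, then starts or stops the timer-driven flag rotation by animation ID.
; Destroying animations also clears that timer after the parent cleanup.
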(event EventBeginPlay
  (CallFunction|Inicializar "/Game/Assets/Materiales/MisMateriales/M_RojoAlgoDañado.M_RojoAlgoDañado" "/Game/Assets/Materiales/MisMateriales/M_RojoAlgoDañado.M_RojoAlgoDañado" "/Game/Assets/Materiales/MisMateriales/M_RojoMuyDañado.M_RojoMuyDañado" "/Game/Assets/Materiales/MisMateriales/M_RojoMuyDañado.M_RojoMuyDañado")
  (Default|Inicializar (Variables|Default|GetRotar%20Bandera) (Variables|Default|GetBandera) 6e+01))

(event EventDestruirAnimaciones
  (|CallParentFunction)
  (Default|BorrarTimer (Variables|Default|GetRotar%20Bandera)))

(fn ConstructionScript)

(fn ElegirAnimacion
  (params (Id :type Integer))
  (bind _rotar_bandera (Variables|Default|GetRotar%20Bandera))
  (|CallParentFunction Id)
  (switch int Id
    (:1
      (Default|CrearTimer _rotar_bandera "Rotar Componente"))
    (:2
      (Default|BorrarTimer _rotar_bandera))))