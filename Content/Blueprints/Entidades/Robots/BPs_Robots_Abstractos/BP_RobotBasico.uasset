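; BP_RobotBasico is a basic robot Blueprint in the abstract robots folder that manages its deterioration, death, wheel and laser-shot animations.
; Inicializar passes meshes, materials and movement values to four animation helper objects.
; RealizarAnimacion forwards an integer ID to ElegirAnimacion, which starts one-off damage or shot animations, or starts and stops timer-driven death and wheel animations.
; DestruirAnimaciones clears the laser, death and wheel timers.
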(event Custom|Inicializar
  (params (Cuerpo%20Medio%20Dañado :type Material%20Interface%20Object%20Reference) (Lado%20Medio%20Dañado :type Material%20Interface%20Object%20Reference) (Cuerpo%20Muy%20Dañado :type Material%20Interface%20Object%20Reference) (Lado%20Muy%20Dañado :type Material%20Interface%20Object%20Reference))
  (Default|Inicializar (Variables|Default|GetAnim%20Deterioro) Cuerpo%20Medio%20Dañado Lado%20Medio%20Dañado Cuerpo%20Muy%20Dañado Lado%20Muy%20Dañado (Variables|Default|GetCuerpoBase))
  (Default|Inicializar (Variables|Default|GetAnim%20Cara%20Laser) (Variables|Default|GetMeshDisparador) 0 "/Game/Assets/Materiales/MisMateriales/M_Rojo.M_Rojo")
  (Default|Inicializar (Variables|Default|GetAnim%20Mover%20Rueda) (Variables|Default|GetMeshDesplazador) (Variables|Default|GetVelocidadBase) 59.0)
  (Default|Inicializar (Variables|Default|GetAnimar%20Muerte) (Variables|Default|GetPosicionBase)))

(event EventDestruirAnimaciones
  (Default|BorrarTimer (Variables|Default|GetAnim%20Cara%20Laser))
  (Default|BorrarTimer (Variables|Default|GetAnimar%20Muerte))
  (Default|BorrarTimer (Variables|Default|GetAnim%20Mover%20Rueda)))

(event EventRealizarAnimacion
  (params (Animacion :type Integer))
  (CallFunction|ElegirAnimacion Animacion))

(fn ConstructionScript)

(fn ElegirAnimacion
  (params (Id :type Integer))
  (bind _anim_deterioro (Variables|Default|GetAnim%20Deterioro))
  (bind _anim_mover_rueda (Variables|Default|GetAnim%20Mover%20Rueda))
  (switch int Id
    (:-2
      (Default|CrearAnimacionSinTimer _anim_deterioro "Deterioro Medio" 0.01))
    (:-1
      (Default|CrearAnimacionSinTimer _anim_deterioro "Deterioro Alto" 0.01))
    (:0
      (Default|CrearTimer (Variables|Default|GetAnimar%20Muerte) "Animar Muerte"))
    (:1
      (Default|CrearTimer _anim_mover_rueda "Rotar Rueda"))
    (:2
      (Default|BorrarTimer _anim_mover_rueda))
    (:3
      (Default|CrearAnimacionSinTimer (Variables|Default|GetAnim%20Cara%20Laser) "Disparo" 0.2))))