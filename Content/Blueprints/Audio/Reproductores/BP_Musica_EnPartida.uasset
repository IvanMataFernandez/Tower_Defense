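; In-match audio player that plays music tracks and a global first-wave sound effect through two separate audio components.
; Events wrap the functions: TocarMusica maps an Id to tracks for match phases, selection, countdown, reaching a target, defeat or victory.
; Both play functions read their volume from the BP_Guardador "save" slot before playing.
; ActualizarVolumen applies given music and SFX volumes, while SetVolumen feeds it the saved values.
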(event Custom|Sonar%20Musica
  (params (Id :type Integer))
  (CallFunction|TocarMusica Id))

(event Custom|Actualizar%20Vol
  (params (Vol%20Musica :type Float%20%28double-precision%29) (Vol%20SFX :type Float%20%28double-precision%29))
  (CallFunction|ActualizarVolumen Vol%20Musica Vol%20SFX))

(event Custom|Sonar%20Efecto%20Global
  (CallFunction|SonarEfecto))

(fn ConstructionScript)

(fn TocarMusica
  (params (Id :type Integer))
  (bind _audiocomponent (Variables|Components|GetAudioComponent))
  (switch int Id
    (:0
      (LocalVariables|SetA%20Tocar (Variables|Default|GetMusica%20Inicio)))
    (:1
      (LocalVariables|SetA%20Tocar (Variables|Default|GetMusica%20Medio)))
    (:2
      (LocalVariables|SetA%20Tocar (Variables|Default|GetMusica%20Fin)))
    (:3
      (LocalVariables|SetA%20Tocar (Variables|Default|GetMusica%20Seleccion)))
    (:4
      (LocalVariables|SetA%20Tocar (Variables|Default|GetCuenta%20Atras)))
    (:5
      (LocalVariables|SetA%20Tocar (Variables|Default|GetMusica%20Llega%20A%20Target)))
    (:6
      (LocalVariables|SetA%20Tocar (Variables|Default|GetMusica%20Derrota)))
    (:7
      (LocalVariables|SetA%20Tocar (Variables|Default|GetMusica%20Victoria))))
  (Audio|Components|Audio|SetSound _audiocomponent (LocalVariables|GetA%20Tocar))
  (bind _returnvalue (SaveGame|LoadGamefromSlot "save"))
  (bind _asbp_guardador (Utilities|Casting|CastToBP_Guardador _returnvalue))
  (Audio|Components|Audio|SetVolumeMultiplier _audiocomponent (Variables|/Script/Tower_Defense.Guardador|GetVolumenAudio _asbp_guardador) :!class /Script/Engine.AudioComponent)
  (Audio|Components|Audio|Play _audiocomponent 0.0)
  (return))

(fn SonarEfecto
  (bind _efectos_globales (Variables|Default|GetEfectos%20Globales))
  (Audio|Components|Audio|SetSound _efectos_globales (Variables|Default|GetEfecto%20Primera%20Oleada))
  (bind _returnvalue (SaveGame|LoadGamefromSlot "save"))
  (bind _asbp_guardador (Utilities|Casting|CastToBP_Guardador _returnvalue))
  (Audio|Components|Audio|SetVolumeMultiplier _efectos_globales (Variables|/Script/Tower_Defense.Guardador|GetVolumenSFX _asbp_guardador) :!class /Script/Engine.AudioComponent)
  (Audio|Components|Audio|Play _efectos_globales 0.0)
  (return))

(fn ActualizarVolumen
  (params (Vol%20Musica :type Float%20%28double-precision%29) (Vol%20SFX :type Float%20%28double-precision%29))
  (Audio|Components|Audio|SetVolumeMultiplier (Variables|Components|GetAudioComponent) Vol%20Musica :!class /Script/Engine.AudioComponent)
  (Audio|Components|Audio|SetVolumeMultiplier (Variables|Default|GetEfectos%20Globales) Vol%20SFX :!class /Script/Engine.AudioComponent)
  (return))

(fn SetVolumen
  (bind _returnvalue (SaveGame|LoadGamefromSlot "save"))
  (bind _asbp_guardador (Utilities|Casting|CastToBP_Guardador _returnvalue))
  (CallFunction|ActualizarVolumen (Variables|/Script/Tower_Defense.Guardador|GetVolumenAudio _asbp_guardador) (Variables|/Script/Tower_Defense.Guardador|GetVolumenSFX _asbp_guardador))
  (return))