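; Helper Blueprint that swaps a basic robot's body materials to show visual deterioration.
; Inicializar caches the body component plus medium and heavy wear materials for the body and sides.
; DeterioroMedio and DeterioroAlto apply the matching set across four material slots, sides on the outer indices and body on the middle two.
; It holds no damage logic; the event graph is unused.
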(event EventBeginPlay
  (|CallParentFunction) ; This node is disabled and will not be called.\nDrag off pins to build functionality.
)

(event EventTick
  (params (DeltaSeconds :type Float%20%28single-precision%29)))

(fn Inicializar
  (params (CuerpoMedio :type Material%20Interface%20Object%20Reference) (LadoMedio :type Material%20Interface%20Object%20Reference) (CuerpoMucho :type Material%20Interface%20Object%20Reference) (LadoMucho :type Material%20Interface%20Object%20Reference) (Cuerpo :type Static%20Mesh%20Component%20Object%20Reference))
  (Variables|Default|SetMaterialMidCuerpo CuerpoMedio)
  (Variables|Default|SetMaterialMidLados LadoMedio)
  (Variables|Default|SetMaterialMuyCuerpo CuerpoMucho)
  (Variables|Default|SetMaterialMuyLados LadoMucho)
  (Variables|Default|SetCuerpo Cuerpo))

(fn DeterioroMedio
  (bind _cuerpo (Variables|Default|GetCuerpo))
  (bind _materialmidlados (Variables|Default|GetMaterialMidLados))
  (bind _materialmidcuerpo (Variables|Default|GetMaterialMidCuerpo))
  (Rendering|Material|SetMaterial _cuerpo 0 _materialmidlados)
  (Rendering|Material|SetMaterial _cuerpo 1 _materialmidcuerpo)
  (Rendering|Material|SetMaterial _cuerpo 2 _materialmidcuerpo)
  (Rendering|Material|SetMaterial _cuerpo 3 _materialmidlados))

(fn DeterioroAlto
  (bind _cuerpo (Variables|Default|GetCuerpo))
  (bind _materialmuylados (Variables|Default|GetMaterialMuyLados))
  (bind _materialmuycuerpo (Variables|Default|GetMaterialMuyCuerpo))
  (Rendering|Material|SetMaterial _cuerpo 0 _materialmuylados)
  (Rendering|Material|SetMaterial _cuerpo 1 _materialmuycuerpo)
  (Rendering|Material|SetMaterial _cuerpo 2 _materialmuycuerpo)
  (Rendering|Material|SetMaterial _cuerpo 3 _materialmuylados))