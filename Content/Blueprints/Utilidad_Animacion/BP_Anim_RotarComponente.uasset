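; BP_Anim_RotarComponente is an animation utility Blueprint that spins a given component around its local yaw axis.
; Inicializar stores the target component and rotation speed, then calls IncializarAudio, which is not defined in this graph.
; RotarComponente adds a local yaw rotation of DeltaTime times the speed on each call.
; BeginPlay and Tick are disabled, so rotation depends on external calls.
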(event EventBeginPlay
  (|CallParentFunction) ; This node is disabled and will not be called.\nDrag off pins to build functionality.
)

(event EventTick
  (params (DeltaSeconds :type Float%20%28single-precision%29))
  (|CallParentFunction DeltaSeconds) ; This node is disabled and will not be called.\nDrag off pins to build functionality.
)

(fn Inicializar
  (params (Componente :type Static%20Mesh%20Component%20Object%20Reference) (VelocidadRotacion :type Float%20%28double-precision%29))
  (Variables|Default|SetComponente Componente)
  (Variables|Default|SetVelocidadRotacion VelocidadRotacion)
  (CallFunction|IncializarAudio))

(fn RotarComponente
  (LocalVariables|SetRotacion (* (Variables|Default|GetDeltaTime) (Variables|Default|GetVelocidadRotacion)))
  (Transformation|AddLocalRotation (Variables|Default|GetComponente) (Math|Rotator|MakeRotator 0.0 0.0 (LocalVariables|GetRotacion)) false false))