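; Animation utility Blueprint that plays the armed ("Preparado") animation of a mine.
; Inicializar stores the mine's tip component, a material slot and the ready material.
; While a one-second timer runs, Preparado raises the tip along relative Z, scaled by delta time, except on frame 12, when it swaps the material instead.
; It increments the timer each call and clears it once the second has passed.
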(event EventBeginPlay
  (|CallParentFunction) ; This node is disabled and will not be called.\nDrag off pins to build functionality.
)

(event EventTick
  (params (DeltaSeconds :type Float%20%28single-precision%29))
  (|CallParentFunction DeltaSeconds) ; This node is disabled and will not be called.\nDrag off pins to build functionality.
)

(fn Inicializar
  (params (Punta :type Static%20Mesh%20Component%20Object%20Reference) (PosMaterial :type Integer) (MaterialPreparado :type Material%20Interface%20Object%20Reference))
  (Variables|Default|SetPuntaDeMina Punta)
  (Variables|Default|SetMaterialPreparado MaterialPreparado)
  (Variables|Default|SetPosMaterial PosMaterial))

(fn Preparado
  (bind _puntademina (Variables|Default|GetPuntaDeMina))
  (bind _relativelocation (Variables|/Script/Engine.SceneComponent|GetRelativeLocation _puntademina))
  (if (.No%20ha%20pasado (CallFunction|ComprobarTimer 1.0))
    (if (== (Variables|Default|GetNumero%20De%20Frame) 12)
      (Rendering|Material|SetMaterial (Variables|Default|GetPuntaDeMina) (Variables|Default|GetPosMaterial) (Variables|Default|GetMaterialPreparado))
      (else
        (Transformation|SetRelativeLocation _puntademina (Math|Vector|MakeVector (.x _relativelocation) (.y _relativelocation) (+ (.z _relativelocation) (* (Variables|Default|GetDeltaTime) 3e+01))) false false)))
    (CallFunction|IncrementarTimer)
    (else
      (CallFunction|BorrarTimer))))