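; Animation utility component that drives code-based animations with named-function timers and plays sounds on its owner.
; CrearTimer resets the counters and starts a looping timer at twice the frame delta sampled once at BeginPlay; another function schedules one-shot calls.
; IncrementarTimer advances elapsed time and frame count, which the Comprobar functions test against targets.
; Audio helpers cache the owner's first AudioComponent to play or deactivate sounds.
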(event EventBeginPlay
  (Variables|Default|SetDeltaTime (* (Utilities|Time|GetWorldDeltaSeconds) 2.0)))

(fn CrearTimer
  (params (Nombre%20Funcion :type String))
  (CallFunction|BorrarTimer)
  (Variables|Default|SetNumeroDeFrame 0)
  (Variables|Default|SetContador 0.0)
  (bind _returnvalue (Utilities|Time|SetTimerbyFunctionName 0 Nombre%20Funcion (Variables|Default|GetDeltaTime) true))
  (Variables|Default|SetTimerAnimacion _returnvalue))

(fn CrearAnimacionSinTimer
  (params (NombreFuncion :type String) (ProgramadoPara :type Float%20%28double-precision%29))
  (Utilities|Time|SetTimerbyFunctionName 0 NombreFuncion ProgramadoPara))

(fn ComprobarTimer
  (params (Target :type Float%20%28double-precision%29))
  (bind _contador (Variables|Default|GetContador))
  (bind _returnvalue (>= _contador Target))
  (return _returnvalue (not _returnvalue)))

(fn BorrarTimer
  (Utilities|Time|ClearandInvalidateTimerbyHandle (Variables|Default|GetTimerAnimacion)))

(fn IncrementarTimer
  (Variables|Default|SetContador (+ (Variables|Default|GetContador) (Variables|Default|GetDeltaTime)))
  (Math|Integer|IncrementInt (Variables|Default|GetNumeroDeFrame)))

(fn ComprobarFrame
  (params (Tiempo :type Integer))
  (bind _numerodeframe (Variables|Default|GetNumeroDeFrame))
  (bind _returnvalue (>= _numerodeframe Tiempo))
  (return _returnvalue (not _returnvalue)))

(fn PararAudio
  (bind _sonido (Variables|Default|GetSonido))
  (if (Utilities|IsValid _sonido)
    (Components|Activation|SetActive _sonido false false)))

(fn IncializarAudio
  (bind _returnvalue (Components|GetOwner))
  (bind _returnvalue_2 (Actor|GetComponentsByClass _returnvalue "/Script/Engine.AudioComponent"))
  (if (not (== (Utilities|Array|Length _returnvalue_2) 0))
    (Variables|Default|SetSonido (Utilities|Array|Get(acopy) _returnvalue_2))
    (return)))

(fn SonarAudio
  (params (Audio :type Sound%20Base%20Object%20Reference))
  (bind _sonido (Variables|Default|GetSonido))
  (Audio|Components|Audio|SetSound _sonido Audio)
  (Audio|Components|Audio|Play _sonido 0.0)
  (return))

(fn ObtenerDeltaTime
  (return (Variables|Default|GetDeltaTime)))

(fn ObtenerFrame
  (return (Variables|Default|GetNumeroDeFrame)))