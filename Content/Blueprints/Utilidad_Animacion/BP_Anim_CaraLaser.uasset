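; Animation helper for a laser face component, apparently on a turret, handling firing, aiming and un-aiming.
; Firing plays a laser sound and briefly swaps in the attack material, restored by a delayed call.
; Aim and un-aim are timer-stepped, delta-time slides along relative Y: out fast to zero, restoring the original material, and back slower.
; Un-aim applies its turret-specific material before moving, gated by a frame check; timer and audio helpers come from outside this file.
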(event EventBeginPlay
  (|CallParentFunction) ; This node is disabled and will not be called.\nDrag off pins to build functionality.
)

(event EventTick
  (params (DeltaSeconds :type Float%20%28single-precision%29))
  (|CallParentFunction DeltaSeconds) ; This node is disabled and will not be called.\nDrag off pins to build functionality.
)

(fn Inicializar
  (params (Componente :type Static%20Mesh%20Component%20Object%20Reference) (Pos%20Material :type Integer) (Material%20Ataque :type Material%20Object%20Reference) (Material%20Desapuntar%20%28Exclusivo%20Torre%29 :type Material%20Interface%20Object%20Reference))
  (Variables|Default|SetCaraLaser Componente)
  (Variables|Default|SetPos%20Material Pos%20Material)
  (Variables|Default|SetMaterial%20Original (Rendering|Material|GetMaterial Componente Pos%20Material))
  (Variables|Default|SetMaterial%20Ataque Material%20Ataque)
  (Variables|Default|SetMaterial%20Desapuntar%20%28Torre%29 Material%20Desapuntar%20%28Exclusivo%20Torre%29)
  (CallFunction|IncializarAudio))

(fn Disparo
  (CallFunction|SonarAudio "/Game/Blueprints/Audio/SFX/Disparo_Laser.Disparo_Laser")
  (Rendering|Material|SetMaterial (Variables|Default|GetCaraLaser) (Variables|Default|GetPos%20Material) (Variables|Default|GetMaterial%20Ataque))
  (CallFunction|CrearAnimacionSinTimer "Disparo Off" 0.2))

(fn DisparoOff
  (Rendering|Material|SetMaterial (Variables|Default|GetCaraLaser) (Variables|Default|GetPos%20Material) (Variables|Default|GetMaterial%20Original)))

(fn Apuntar
  (bind _deltatime (CallFunction|ObtenerDeltaTime))
  (bind _caralaser (Variables|Default|GetCaraLaser))
  (bind _caralaser_2 (Variables|Default|GetCaraLaser))
  (bind _returnvalue (* 3e+03 _deltatime))
  (bind _relativelocation (Variables|/Script/Engine.SceneComponent|GetRelativeLocation _caralaser_2))
  (bind _returnvalue_2 (+ (.y _relativelocation) _returnvalue))
  (if (>= _returnvalue_2 0.0)
    (Transformation|SetRelativeLocation _caralaser "0, 0, 0" false false)
    (Rendering|Material|SetMaterial (Variables|Default|GetCaraLaser) (Variables|Default|GetPos%20Material) (Variables|Default|GetMaterial%20Original))
    (CallFunction|BorrarTimer)
    (else
      (Transformation|SetRelativeLocation _caralaser (Math|Vector|MakeVector 0.0 _returnvalue_2 0.0) false false)
      (CallFunction|IncrementarTimer))))

(fn Desapuntar
  (bind _deltatime (CallFunction|ObtenerDeltaTime))
  (bind _caralaser (Variables|Default|GetCaraLaser))
  (bind _caralaser_2 (Variables|Default|GetCaraLaser))
  (bind _returnvalue (* -3e+02 _deltatime))
  (bind _relativelocation (Variables|/Script/Engine.SceneComponent|GetRelativeLocation _caralaser))
  (bind _returnvalue_2 (+ (.y _relativelocation) _returnvalue))
  (if (.Ha%20pasado (CallFunction|ComprobarFrame 2))
    (if (<= _returnvalue_2 -228.0)
      (Transformation|SetRelativeLocation _caralaser_2 "0,-228.000000, 0" false false)
      (CallFunction|BorrarTimer)
      (else
        (Transformation|SetRelativeLocation _caralaser_2 (Math|Vector|MakeVector 0.0 _returnvalue_2 0.0) false false)
        (CallFunction|IncrementarTimer)))
    (else
      (Rendering|Material|SetMaterial (Variables|Default|GetCaraLaser) (Variables|Default|GetPos%20Material) (Variables|Default|GetMaterial%20Desapuntar%20%28Torre%29))
      (CallFunction|IncrementarTimer))))