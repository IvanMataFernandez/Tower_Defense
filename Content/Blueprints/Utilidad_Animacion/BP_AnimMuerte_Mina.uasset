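; Death animation helper for a mine, driving a tip component and a body component passed in through Inicializar.
; AnimarMuerte plays a tower death sound behind a frame check, then shrinks the body and lowers the tip along relative Z using DeltaTime while a short timer runs.
; It advances the timer itself and clears it once the time has passed, so the animation relies on repeated calls rather than a Timeline.
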(fn Inicializar
  (params (Punta :type Static%20Mesh%20Component%20Object%20Reference) (Cuerpo :type Static%20Mesh%20Component%20Object%20Reference))
  (Variables|Default|SetPunta%20De%20Mina Punta)
  (Variables|Default|SetCuerpo Cuerpo))

(fn AnimarMuerte
  (bind _cuerpo (Variables|Default|GetCuerpo))
  (bind _punta_de_mina (Variables|Default|GetPunta%20De%20Mina))
  (bind _relativelocation (Variables|/Script/Engine.SceneComponent|GetRelativeLocation _punta_de_mina))
  (if (.No%20ha%20pasado (CallFunction|ComprobarFrame 1))
    (CallFunction|SonarAudio "/Game/Blueprints/Audio/SFX/Torre_Muerte2.Torre_Muerte2"))
  (if (.No%20ha%20pasado (CallFunction|ComprobarTimer 1.0))
    (Transformation|SetRelativeScale3D _cuerpo (- (Variables|/Script/Engine.SceneComponent|GetRelativeScale3D _cuerpo) (* (Variables|Default|GetDeltaTime) 0.5)))
    (Transformation|SetRelativeLocation _punta_de_mina (Math|Vector|MakeVector (.x _relativelocation) (.y _relativelocation) (- (.z _relativelocation) (* (Variables|Default|GetDeltaTime) 1e+01))) false false)
    (CallFunction|IncrementarTimer)
    (else
      (CallFunction|BorrarTimer))))