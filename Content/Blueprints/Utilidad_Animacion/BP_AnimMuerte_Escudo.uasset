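; Death animation utility for a shield unit, apparently a tower, that tips its base over when it dies.
; Inicializar stores the shield component and base and sets up audio.
; AnimarMuerte advances per call: before the first-frame check passes it plays the death sound and hides the shield.
; It decreases the base's roll at a delta-time-scaled rate until near -90 degrees, then snaps the rotation and clears the timer.
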(event EventBeginPlay
  (|CallParentFunction) ; This node is disabled and will not be called.\nDrag off pins to build functionality.
)

(event EventTick
  (params (DeltaSeconds :type Float%20%28single-precision%29)))

(fn Inicializar
  (params (Componente%20Escudo :type BP%20Anim%20Rotar%20Componente%20Object%20Reference) (Base :type Static%20Mesh%20Component%20Object%20Reference))
  (Variables|Default|SetEscudo Componente%20Escudo)
  (Variables|Default|SetBase Base)
  (CallFunction|IncializarAudio))

(fn AnimarMuerte
  (bind _deltatime (CallFunction|ObtenerDeltaTime))
  (bind _base (Variables|Default|GetBase))
  (bind _returnvalue (* _deltatime 1.3e+02))
  (bind _relativerotation (Variables|/Script/Engine.SceneComponent|GetRelativeRotation _base))
  (bind _returnvalue_2 (- (.roll _relativerotation) _returnvalue))
  (if (.Ha%20pasado (CallFunction|ComprobarFrame 1))
    (if (> _returnvalue_2 -9e+01)
      (Transformation|SetRelativeRotation _base (Math|Rotator|MakeRotator _returnvalue_2 (.pitch _relativerotation) (.yaw _relativerotation)) false false :!label _label)
      (CallFunction|IncrementarTimer)
      (else
        (Transformation|SetRelativeRotation _base "0.0,0.0,-90.000000" false false)
        (CallFunction|BorrarTimer)))
    (else
      (CallFunction|SonarAudio "/Game/Blueprints/Audio/SFX/Torre_Muerte1.Torre_Muerte1")
      (Default|OcultarComponente (Variables|Default|GetEscudo))
      (goto _label))))