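; Animation utility Blueprint for the death of a double-panel piece, apparently on a tower, tilting the panels and playing a death sound.
; Inicializar stores the Paneles component and sets up audio.
; Each AnimarMuerte call raises relative pitch at 60 degrees per second, clamping at 50 and zeroing roll and yaw.
; A frame check gates the sound to the start, with the timer incremented during the tilt and cleared at the limit.
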(event EventBeginPlay
  (|CallParentFunction) ; This node is disabled and will not be called.\nDrag off pins to build functionality.
)

(event EventTick
  (params (DeltaSeconds :type Float%20%28single-precision%29))
  (|CallParentFunction DeltaSeconds) ; This node is disabled and will not be called.\nDrag off pins to build functionality.
)

(fn Inicializar
  (params (Paneles :type Static%20Mesh%20Component%20Object%20Reference))
  (Variables|Default|SetPaneles Paneles)
  (CallFunction|IncializarAudio))

(fn AnimarMuerte
  (bind _deltatime (CallFunction|ObtenerDeltaTime))
  (bind _paneles (Variables|Default|GetPaneles))
  (bind _paneles_2 (Variables|Default|GetPaneles))
  (bind _returnvalue (* _deltatime 6e+01))
  (bind _relativerotation (Variables|/Script/Engine.SceneComponent|GetRelativeRotation _paneles_2))
  (bind _returnvalue_2 (+ (.pitch _relativerotation) _returnvalue))
  (if (.No%20ha%20pasado (CallFunction|ComprobarFrame 1))
    (CallFunction|SonarAudio "/Game/Blueprints/Audio/SFX/Torre_Muerte2.Torre_Muerte2"))
  (if (<= _returnvalue_2 5e+01)
    (Transformation|SetRelativeRotation _paneles (Math|Rotator|MakeRotator 0.0 _returnvalue_2 0.0) false false)
    (CallFunction|IncrementarTimer)
    (else
      (Transformation|SetRelativeRotation _paneles "50.000000,0.0,0.0" false false)
      (CallFunction|BorrarTimer))))