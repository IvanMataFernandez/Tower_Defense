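; Animation helper for panels that switches material slot 2 of a component between red and blue for a "producir" (produce) animation.
; Inicializar stores the target component, and AnimarProducir advances the animation each time it is called.
; It shows red and increments a timer until a short threshold passes, then shows blue and clears the timer.
; Event Tick is disabled, so the animation relies on external calls.
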(event EventBeginPlay
  (|CallParentFunction) ; This node is disabled and will not be called.\nDrag off pins to build functionality.
)

(event EventTick
  (params (DeltaSeconds :type Float%20%28single-precision%29))
  (|CallParentFunction DeltaSeconds) ; This node is disabled and will not be called.\nDrag off pins to build functionality.
)

(fn AnimarProducir
  (bind _componente (Variables|Default|GetComponente))
  (if (.No%20ha%20pasado (CallFunction|ComprobarTimer 0.1))
    (Rendering|Material|SetMaterial _componente 2 "/Game/Assets_Mios/Materiales/M_Rojo.M_Rojo")
    (CallFunction|IncrementarTimer)
    (else
      (Rendering|Material|SetMaterial _componente 2 "/Game/Assets_Mios/Materiales/M_Azul.M_Azul")
      (CallFunction|BorrarTimer))))

(fn Inicializar
  (params (Componente :type Static%20Mesh%20Component%20Object%20Reference))
  (CallFunction|SetComponente Componente))