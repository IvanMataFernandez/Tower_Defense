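; Animation utility Blueprint that plays a bomb's detonation countdown and explosion on a component passed to Inicializar.
; AnimarCountdownExplosion advances a timer per call, playing countdown audio at the start and toggling flash material and scale pulse at fixed intervals.
; When time runs out, it plays explosion audio, spawns particles (larger with smoke for big explosions) and clears the timer.
; Timer and audio helpers are defined outside this graph; its own Tick is disabled.
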(event EventBeginPlay
  (|CallParentFunction) ; This node is disabled and will not be called.\nDrag off pins to build functionality.
)

(event EventTick
  (params (DeltaSeconds :type Float%20%28single-precision%29))
  (|CallParentFunction DeltaSeconds) ; This node is disabled and will not be called.\nDrag off pins to build functionality.
)

(fn Inicializar
  (params (Componente :type Static%20Mesh%20Component%20Object%20Reference) (Pos%20Material :type Integer) (Material%20Flash :type Material%20Interface%20Object%20Reference) (Tiempo%20De%20Animacion :type Float%20%28double-precision%29) (Explosion%20Grande :type Boolean))
  (Variables|Default|SetCuerpoBomba Componente)
  (Variables|Default|SetPos%20Material Pos%20Material)
  (Variables|Default|SetMaterial%20Original (Rendering|Material|GetMaterial (Variables|Default|GetCuerpoBomba) Pos%20Material))
  (Variables|Default|SetMaterial%20Flash Material%20Flash)
  (Variables|Default|SetEstadoTick 1)
  (Variables|Default|SetTiempoDeAnimacion Tiempo%20De%20Animacion)
  (Variables|Default|SetExplosion%20Grande Explosion%20Grande)
  (CallFunction|IncializarAudio))

(fn AnimarCountdownExplosion
  (bind _cuerpobomba (Variables|Default|GetCuerpoBomba))
  (bind _returnvalue (Transformation|GetWorldLocation _cuerpobomba))
  (if (.No%20ha%20pasado (CallFunction|ComprobarFrame 1))
    (CallFunction|SonarAudio "/Game/Blueprints/Audio/SFX/Cuenta_Atras_Bomba.Cuenta_Atras_Bomba"))
  (if (.No%20ha%20pasado (CallFunction|ComprobarTimer (Variables|Default|GetTiempoDeAnimacion)))
    (Utilities|FlowControl|Sequence
      (:then_0
        (if (.Ha%20pasado (CallFunction|ComprobarTimer (* (Variables|Default|GetEstadoTick) 0.34)))
          (CallFunction|CambiarAparienciaBomba)
          (Math|Integer|IncrementInt (Variables|Default|GetEstadoTick))))
      (:then_1
        (CallFunction|IncrementarTimer)))
    (else
      (CallFunction|SonarAudio "/Game/Blueprints/Audio/SFX/Explosion_Bomba.Explosion_Bomba")
      (if (Variables|Default|GetExplosion%20Grande)
        (Effects|SpawnEmitteratLocation "/Game/Realistic_Starter_VFX_Pack_Vol2/Particles/Explosion/P_Explosion_Big_B.P_Explosion_Big_B" _returnvalue "0, 0, 0" "2.000000,2.000000,2.000000")
        (Effects|SpawnEmitteratLocation "/Game/Realistic_Starter_VFX_Pack_Vol2/Particles/Explosion/P_Explosion_Smoke.P_Explosion_Smoke" _returnvalue "0, 0, 0" "2.000000,2.000000,2.000000")
        (else
          (Effects|SpawnEmitteratLocation "/Game/Realistic_Starter_VFX_Pack_Vol2/Particles/Explosion/P_Explosion_Big_B.P_Explosion_Big_B" _returnvalue)))
      (CallFunction|BorrarTimer))))

(fn CambiarAparienciaBomba
  (bind _output_get (Variables|Default|SetNegro (not (Variables|Default|GetNegro))))
  (CallFunction|CambiarColorBomba _output_get)
  (bind _output_get_2 (Variables|Default|SetAgrandar (not (Variables|Default|GetAgrandar))))
  (CallFunction|CambiarEscalaBomba _output_get_2))

(fn CambiarColorBomba
  (params (Negro :type Boolean))
  (bind _pos_material (Variables|Default|GetPos%20Material))
  (if Negro
    (Rendering|Material|SetMaterial (Variables|Default|GetCuerpoBomba) _pos_material (Variables|Default|GetMaterial%20Original))
    (else
      (Rendering|Material|SetMaterial (Variables|Default|GetCuerpoBomba) _pos_material (Variables|Default|GetMaterial%20Flash))))
  (return))

(fn CambiarEscalaBomba
  (params (Agrandar :type Boolean))
  (if Agrandar
    (Transformation|SetWorldScale3D (Variables|Default|GetCuerpoBomba) (+ (Transformation|GetWorldScale (Variables|Default|GetCuerpoBomba)) "0.200000,0.200000,0.200000"))
    (else
      (Transformation|SetWorldScale3D (Variables|Default|GetCuerpoBomba) (+ (Transformation|GetWorldScale (Variables|Default|GetCuerpoBomba)) "-0.200000,-0.200000,-0.200000"))))
  (return))