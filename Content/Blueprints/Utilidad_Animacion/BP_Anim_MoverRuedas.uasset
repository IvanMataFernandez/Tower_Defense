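; BP_Anim_MoverRuedas is an animation utility that spins a wheel component to match a linear velocity.
; Inicializar stores the component and divides velocity by wheel radius, converts to degrees, scales by DeltaTime and negates it for direction.
; RotarRueda applies that precomputed per-step angle as a relative roll rotation.
; DeltaTime is not assigned in these graphs, and BeginPlay and Tick are disabled.
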(event EventBeginPlay
  (|CallParentFunction) ; This node is disabled and will not be called.\nDrag off pins to build functionality.
)

(event EventTick
  (params (DeltaSeconds :type Float%20%28single-precision%29))
  (|CallParentFunction DeltaSeconds) ; This node is disabled and will not be called.\nDrag off pins to build functionality.
)

(fn Inicializar
  (params (Componente :type Static%20Mesh%20Component%20Object%20Reference) (VelocidadLineal :type Float%20%28double-precision%29) (RadioDeRueda :type Float%20%28double-precision%29))
  (CallFunction|SetComponente Componente)
  (Variables|Default|SetDeltaVelocidadAngular (* (* (* (/ VelocidadLineal RadioDeRueda) (/ 1.8e+02 (Math|Trig|GetPI))) (Variables|Default|GetDeltaTime)) -1.0)))

(fn RotarRueda
  (Transformation|AddRelativeRotation (Variables|Default|GetComponente) (Math|Rotator|MakeRotator (Variables|Default|GetDeltaVelocidadAngular) 0.0 0.0) false false))