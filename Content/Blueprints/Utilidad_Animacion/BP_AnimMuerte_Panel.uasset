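; Animation utility Blueprint that plays the death animation of a Panel component, judging by the sound name part of a tower.
; Inicializar stores the panel and sets up audio.
; AnimarMuerte advances per call using delta time: it plays the death sound at the start, lowers the panel to a Z limit, then rolls it over.
; Helper calls increment a timer during motion and clear it when finished.
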(event EventBeginPlay
  (|CallParentFunction) ; This node is disabled and will not be called.\nDrag off pins to build functionality.
)

(event EventTick
  (params (DeltaSeconds :type Float%20%28single-precision%29))
  (|CallParentFunction DeltaSeconds) ; This node is disabled and will not be called.\nDrag off pins to build functionality.
)

(fn Inicializar
  (params (Panel :type Static%20Mesh%20Component%20Object%20Reference))
  (Variables|Default|SetPanel Panel)
  (CallFunction|IncializarAudio))

(fn AnimarMuerte
  (bind _deltatime (CallFunction|ObtenerDeltaTime))
  (bind _panel (Variables|Default|GetPanel))
  (bind _panel_2 (Variables|Default|GetPanel))
  (bind _returnvalue (* _deltatime 4e+02))
  (bind _relativelocation (Variables|/Script/Engine.SceneComponent|GetRelativeLocation _panel))
  (bind _relativerotation (Variables|/Script/Engine.SceneComponent|GetRelativeRotation _panel_2))
  (bind _returnvalue_2 (- (.z _relativelocation) _returnvalue))
  (if (.Ha%20pasado (CallFunction|ComprobarFrame 1))
    _
    (else
      (CallFunction|SonarAudio "/Game/Blueprints/Audio/SFX/Torre_Muerte1.Torre_Muerte1")))
  (if (>= (.z _relativelocation) -184.0)
    (bind _result (Math|Float|NegateFloat _returnvalue_2)
      (:%20%20
        (Transformation|SetRelativeLocation (Variables|Default|GetPanel) (Math|Vector|MakeVector 0.0 _result _returnvalue_2) false false)
        (CallFunction|IncrementarTimer :!label _label)))
    (elif (>= (.roll _relativerotation) -44.0)
      (Transformation|SetRelativeRotation (Variables|Default|GetPanel) (Math|Rotator|MakeRotator (+ (.roll _relativerotation) (* (CallFunction|ObtenerDeltaTime) -1.2e+02)) 0.0 0.0) false false)
      (goto _label)
      (else
        (CallFunction|BorrarTimer)))))