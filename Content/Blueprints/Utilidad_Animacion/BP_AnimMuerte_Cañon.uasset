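; Death animation helper for a cannon tower that tips the tower's face component over when it dies.
; Inicializar stores the Cara component to animate.
; AnimarMuerte plays a death sound on a frame check, then lowers Cara's roll at a delta-time-scaled constant rate, advancing the timer each step.
; Once the roll reaches its sideways limit, it snaps there and clears the timer.
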(event EventBeginPlay
  (|CallParentFunction) ; This node is disabled and will not be called.\nDrag off pins to build functionality.
)

(event EventTick
  (params (DeltaSeconds :type Float%20%28single-precision%29))
  (|CallParentFunction DeltaSeconds) ; This node is disabled and will not be called.\nDrag off pins to build functionality.
)

(fn AnimarMuerte
  (bind _deltatime (Variables|Default|GetDeltaTime))
  (bind _cara (Variables|Default|GetCara))
  (bind _returnvalue (* 1e+02 _deltatime))
  (bind _relativerotation (Variables|/Script/Engine.SceneComponent|GetRelativeRotation _cara))
  (bind _returnvalue_2 (- (.roll _relativerotation) _returnvalue))
  (if (.No%20ha%20pasado (CallFunction|ComprobarFrame 1))
    (CallFunction|SonarAudio "/Game/Blueprints/Audio/SFX/Torre_Muerte1.Torre_Muerte1"))
  (if (<= _returnvalue_2 -9e+01)
    (Transformation|SetRelativeRotation _cara "0, 0,-90.000000" false false)
    (CallFunction|BorrarTimer)
    (else
      (Transformation|SetRelativeRotation (Variables|Default|GetCara) (Math|Rotator|MakeRotator _returnvalue_2 0.0 0.0) false false)
      (CallFunction|IncrementarTimer))))

(fn Inicializar
  (params (Cara :type Static%20Mesh%20Component%20Object%20Reference))
  (Variables|Default|SetCara Cara))