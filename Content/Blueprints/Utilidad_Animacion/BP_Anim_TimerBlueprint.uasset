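; Animation utility component that gives other objects a timer for stepping animations, plus helpers for playing sound.
; It starts a looping, fixed-interval timer or a one-shot one, calling a function by name on the supplied object.
; A manually incremented time and frame counter lets callers test whether a target has passed.
; Audio helpers use the owner's first AudioComponent to play or stop sounds, or play them as 2D.
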(event EventBeginPlay
  (Variables|Default|SetDeltaTime (* 0.016 2.0)))

(fn CrearTimer
  (params (Nombre%20Funcion :type String) (Comp%20Animacion :type Actor%20Component%20Object%20Reference))
  (CallFunction|BorrarTimer)
  (Variables|Default|SetNumero%20De%20Frame 0)
  (Variables|Default|SetContador 0.0)
  (bind _returnvalue (Utilities|Time|SetTimerbyFunctionName Comp%20Animacion Nombre%20Funcion (Variables|Default|GetDeltaTime) true))
  (Variables|Default|SetTimer%20Animacion _returnvalue))

(fn CrearAnimacionSinTimer
  (params (NombreFuncion :type String) (CompAnimacion :type Actor%20Component%20Object%20Reference) (ProgramadoPara :type Float%20%28double-precision%29))
  (Utilities|Time|SetTimerbyFunctionName CompAnimacion NombreFuncion ProgramadoPara))

(fn ComprobarTimer
  (params (Target :type Float%20%28double-precision%29))
  (bind _contador (Variables|Default|GetContador))
  (bind _returnvalue (>= _contador Target))
  (return _returnvalue (not _returnvalue)))

(fn BorrarTimer
  (Utilities|Time|ClearandInvalidateTimerbyHandle (Variables|Default|GetTimer%20Animacion)))

(fn IncrementarTimer
  (Variables|Default|SetContador (+ (Variables|Default|GetContador) (Variables|Default|GetDeltaTime)))
  (Math|Integer|IncrementInt (Variables|Default|GetNumero%20De%20Frame)))

(fn ComprobarFrame
  (params (Tiempo :type Integer))
  (bind _numero_de_frame (Variables|Default|GetNumero%20De%20Frame))
  (bind _returnvalue (>= _numero_de_frame Tiempo))
  (return _returnvalue (not _returnvalue)))

(fn PararAudio
  (bind _sonido (Variables|Default|GetSonido))
  (if (Utilities|IsValid _sonido)
    (Components|Activation|SetActive _sonido false false)))

(fn IncializarAudio
  (bind _returnvalue (Components|GetOwner))
  (bind _returnvalue_2 (Actor|GetComponentsByClass _returnvalue "/Script/Engine.AudioComponent"))
  (if (not (== (Utilities|Array|Length _returnvalue_2) 0))
    (Variables|Default|SetSonido (Utilities|Array|Get(acopy) _returnvalue_2))
    (return)))

(fn SonarAudio
  (params (Audio :type Sound%20Base%20Object%20Reference))
  (bind _sonido (Variables|Default|GetSonido))
  (Audio|Components|Audio|SetSound _sonido Audio)
  (Audio|Components|Audio|Play _sonido 0.0)
  (return))

(fn SonarAudioExternamente
  (params (Audio :type Sound%20Base%20Object%20Reference))
  (Audio|PlaySound2D Audio 1.0 1.0 0.0 0 0)
  (return))