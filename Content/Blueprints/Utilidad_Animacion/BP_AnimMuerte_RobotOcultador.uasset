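; BP_AnimMuerte_RobotOcultador is an animation utility that plays the death of the RobotOcultador, splitting its ball shell open.
; Inicializar stores the body and both half-shell components and sets up audio.
; AnimarMuerte plays the death sound and resets transforms on its first frame.
; Delta-time steps then pitch the halves oppositely, derive their sideways slide from that angle and lower the body, clearing the timer once fully open.
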(fn Inicializar
  (params (Cuerpo :type Static%20Mesh%20Component%20Object%20Reference) (Mitad%20Izquierda%20de%20Frente :type Static%20Mesh%20Component%20Object%20Reference) (Mitad%20Derecha%20de%20Frente :type Static%20Mesh%20Component%20Object%20Reference))
  (Variables|Default|SetCuerpo Cuerpo)
  (Variables|Default|SetMitadBola1 Mitad%20Izquierda%20de%20Frente)
  (Variables|Default|SetMitadBola2 Mitad%20Derecha%20de%20Frente)
  (CallFunction|IncializarAudio))

(fn AnimarMuerte
  (bind _deltatime (CallFunction|ObtenerDeltaTime))
  (bind _mitadbola2 (Variables|Default|GetMitadBola2))
  (bind _cuerpo (Variables|Default|GetCuerpo))
  (bind _mitadbola1 (Variables|Default|GetMitadBola1))
  (bind _mitadbola2_2 (Variables|Default|GetMitadBola2))
  (bind _returnvalue (* _deltatime 1.2e+02))
  (bind _relativelocation (Variables|/Script/Engine.SceneComponent|GetRelativeLocation _cuerpo))
  (bind _relativerotation (Variables|/Script/Engine.SceneComponent|GetRelativeRotation _mitadbola2_2))
  (bind _returnvalue_2 (+ _returnvalue (.pitch _relativerotation)))
  (bind _returnvalue_3 (* _returnvalue_2 -3.0))
  (if (.Ha%20pasado (CallFunction|ComprobarFrame 1))
    _
    (else
      (CallFunction|SonarAudio "/Game/Blueprints/Audio/SFX/Muerte_Robot.Muerte_Robot")
      (Transformation|SetRelativeLocation (Variables|Default|GetMitadBola1) "0, 0,141.000000" false false)
      (Transformation|SetRelativeLocation (Variables|Default|GetMitadBola2) "0, 0,141.000000" false false)
      (Transformation|SetRelativeScale3D (Variables|Default|GetCuerpo) "1.000000,1.000000,1.000000")))
  (if (< (.pitch _relativerotation) 85.0)
    (Transformation|SetRelativeRotation _mitadbola2 (Math|Rotator|MakeRotator 0.0 _returnvalue_2 0.0) false false)
    (Transformation|SetRelativeLocation _mitadbola2 (Math|Vector|MakeVector _returnvalue_3 0.0 1.2e+02) false false)
    (Transformation|SetRelativeRotation _mitadbola1 (Math|Rotator|MakeRotator 0.0 (* _returnvalue_2 -1.0) 0.0) false false)
    (Transformation|SetRelativeLocation _mitadbola1 (Math|Vector|MakeVector (* _returnvalue_3 -1.0) 0.0 1.2e+02) false false)
    (if (> (.z _relativelocation) 1.2e+02)
      (Transformation|SetRelativeLocation (Variables|Default|GetCuerpo) (Math|Vector|MakeVector 0.0 0.0 (- (.z _relativelocation) (* (CallFunction|ObtenerDeltaTime) 1e+02))) false false))
    (CallFunction|IncrementarTimer)
    (else
      (CallFunction|BorrarTimer))))