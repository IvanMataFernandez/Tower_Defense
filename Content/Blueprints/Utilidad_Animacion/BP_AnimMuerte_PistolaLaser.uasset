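; Death animation utility for the laser pistol, shrinking it away while playing a tower death sound.
; Inicializar stores the pistol reference and sets up audio.
; Each AnimarMuerte call reduces the scale uniformly at a constant delta-time-based rate, using a frame check to gate the sound to the start.
; It increments the timer while shrinking, then clamps the scale to zero and clears the timer.
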(fn Inicializar
  (params (Pistola :type Static%20Mesh%20Component%20Object%20Reference))
  (Variables|Default|SetPistola Pistola)
  (CallFunction|IncializarAudio))

(fn AnimarMuerte
  (bind _deltatime (CallFunction|ObtenerDeltaTime))
  (bind _pistola (Variables|Default|GetPistola))
  (bind _pistola_2 (Variables|Default|GetPistola))
  (bind _returnvalue (* _deltatime -1.2))
  (bind _relativescale3d (Variables|/Script/Engine.SceneComponent|GetRelativeScale3D _pistola_2))
  (bind _returnvalue_2 (+ (.x _relativescale3d) _returnvalue))
  (if (.No%20ha%20pasado (CallFunction|ComprobarFrame 1))
    (CallFunction|SonarAudio "/Game/Blueprints/Audio/SFX/Torre_Muerte2.Torre_Muerte2"))
  (if (> _returnvalue_2 0.0)
    (Transformation|SetRelativeScale3D _pistola (Math|Vector|MakeVector _returnvalue_2 _returnvalue_2 _returnvalue_2))
    (CallFunction|IncrementarTimer)
    (else
      (Transformation|SetRelativeScale3D _pistola "0, 0, 0")
      (CallFunction|BorrarTimer))))