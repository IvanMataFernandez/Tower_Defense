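; Animation utility Blueprint that switches a hider robot ("RobotOcultador") to its deteriorated look.
; Inicializar stores references to the body, the two ball halves and their damaged materials.
; Deteriorar then sets those damaged materials on slot 0 of each part, as an instant swap with no timeline or blending.
; The event graph has no active logic, so both functions rely on external callers.
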(event EventBeginPlay
  (|CallParentFunction) ; This node is disabled and will not be called.\nDrag off pins to build functionality.
)

(event EventTick
  (params (DeltaSeconds :type Float%20%28single-precision%29)))

(fn Inicializar
  (params (Cuerpo :type Static%20Mesh%20Component%20Object%20Reference) (Mitad%20Bola%201 :type Static%20Mesh%20Component%20Object%20Reference) (Mitad%20Bola%202 :type Static%20Mesh%20Component%20Object%20Reference) (Material%20Cuerpo%20Dañado :type Material%20Interface%20Object%20Reference) (Material%20Bola%20Dañada :type Material%20Interface%20Object%20Reference))
  (Variables|Default|SetCuerpo Cuerpo)
  (Variables|Default|SetMitad%20Bola%201 Mitad%20Bola%201)
  (Variables|Default|SetMitad%20Bola%202 Mitad%20Bola%202)
  (Variables|Default|SetCuerpo%20Dañado Material%20Cuerpo%20Dañado)
  (Variables|Default|SetBola%20Dañada Material%20Bola%20Dañada))

(fn Deteriorar
  (bind _bola_dañada (Variables|Default|GetBola%20Dañada))
  (Rendering|Material|SetMaterial (Variables|Default|GetCuerpo) 0 (Variables|Default|GetCuerpo%20Dañado))
  (Rendering|Material|SetMaterial (Variables|Default|GetMitad%20Bola%201) 0 _bola_dañada)
  (Rendering|Material|SetMaterial (Variables|Default|GetMitad%20Bola%202) 0 _bola_dañada))