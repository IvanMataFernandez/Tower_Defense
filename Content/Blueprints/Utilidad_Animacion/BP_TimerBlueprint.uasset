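; BP_TimerBlueprint is an animation timer utility that drives a named function on a given object at a fixed step.
; CrearTimer zeroes the elapsed counter and starts a looping timer at the DeltaTime interval, keeping its handle for BorrarTimer to clear.
; IncrementarTimer manually advances the counter by that step and counts frames.
; ComprobarTimer reports whether the counter has reached a target.
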(event EventBeginPlay)

(event EventTick
  (params (DeltaSeconds :type Float%20%28single-precision%29)))

(fn ComprobarTimer
  (params (Target :type Float%20%28double-precision%29))
  (bind _contador (Variables|Default|GetContador))
  (bind _returnvalue (>= _contador Target))
  (return _returnvalue (not _returnvalue)))

(fn BorrarTimer
  (Utilities|Time|ClearandInvalidateTimerbyHandle (Variables|Default|GetTimer%20Animacion)))

(fn IncrementarTimer
  (Variables|Default|SetContador (+ (Variables|Default|GetContador) (Variables|Default|GetDeltaTime)))
  (Math|Integer|IncrementInt (Variables|Default|GetNumero%20De%20Frame)))

(fn CrearTimer
  (params (Nombre%20Funcion :type String) (Actor :type Actor%20Object%20Reference))
  (Variables|Default|SetContador 0.0)
  (bind _returnvalue (Utilities|Time|SetTimerbyFunctionName Actor Nombre%20Funcion (Variables|Default|GetDeltaTime) true))
  (Variables|Default|SetTimer%20Animacion _returnvalue))