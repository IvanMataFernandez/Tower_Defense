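; Animation helper for protectors ("Protectores") that hides and reveals a body flanked by two ball halves.
; Inicializar stores the three components.
; Ocultar slides the halves symmetrically apart on X while shrinking the body's X scale to near zero, and Desocultar reverses it.
; Each call advances one delta-time step, calling IncrementarTimer until the travel limit, then snapping to the end pose and calling BorrarTimer.
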(event EventBeginPlay
  (|CallParentFunction) ; This node is disabled and will not be called.\nDrag off pins to build functionality.
)

(event EventTick
  (params (DeltaSeconds :type Float%20%28single-precision%29)))

(fn Inicializar
  (params (Cuerpo :type Static%20Mesh%20Component%20Object%20Reference) (Mitad%20Izquierda%20de%20Frente :type Static%20Mesh%20Component%20Object%20Reference) (Mitad%20Derecha%20de%20Frente :type Static%20Mesh%20Component%20Object%20Reference))
  (Variables|Default|SetCuerpo Cuerpo)
  (Variables|Default|SetMitad%20Bola%201 Mitad%20Izquierda%20de%20Frente)
  (Variables|Default|SetMitad%20Bola%202 Mitad%20Derecha%20de%20Frente))

(fn Ocultar
  (bind _deltatime (CallFunction|ObtenerDeltaTime))
  (bind _mitad_bola_2 (Variables|Default|GetMitad%20Bola%202))
  (bind _returnvalue (* _deltatime 1.6e+02))
  (bind _relativelocation (Variables|/Script/Engine.SceneComponent|GetRelativeLocation _mitad_bola_2))
  (bind _returnvalue_2 (+ (.x _relativelocation) _returnvalue))
  (Transformation|SetRelativeLocation (Variables|Default|GetMitad%20Bola%201) (Math|Vector|MakeVector (* _returnvalue_2 -1.0) 0.0 141.0) false false)
  (Transformation|SetRelativeLocation (Variables|Default|GetMitad%20Bola%202) (Math|Vector|MakeVector _returnvalue_2 0.0 141.0) false false)
  (Transformation|SetRelativeScale3D (Variables|Default|GetCuerpo) (Math|Vector|MakeVector (/ (- 82.0 _returnvalue_2) 82.0) 1.0 1.0))
  (if (< _returnvalue_2 82.0)
    (CallFunction|IncrementarTimer)
    (else
      (Transformation|SetRelativeLocation (Variables|Default|GetMitad%20Bola%201) "-82.000000,0.0,141.000000" false false)
      (Transformation|SetRelativeLocation (Variables|Default|GetMitad%20Bola%202) "82.000000,0.0,141.000000" false false)
      (Transformation|SetRelativeScale3D (Variables|Default|GetCuerpo) "0.001000,1.000000,1.000000")
      (CallFunction|BorrarTimer))))

(fn Desocultar
  (bind _deltatime (CallFunction|ObtenerDeltaTime))
  (bind _mitad_bola_2 (Variables|Default|GetMitad%20Bola%202))
  (bind _returnvalue (* _deltatime 1.6e+02))
  (bind _relativelocation (Variables|/Script/Engine.SceneComponent|GetRelativeLocation _mitad_bola_2))
  (bind _returnvalue_2 (- (.x _relativelocation) _returnvalue))
  (Transformation|SetRelativeLocation (Variables|Default|GetMitad%20Bola%201) (Math|Vector|MakeVector (* _returnvalue_2 -1.0) 0.0 141.0) false false)
  (Transformation|SetRelativeLocation (Variables|Default|GetMitad%20Bola%202) (Math|Vector|MakeVector _returnvalue_2 0.0 141.0) false false)
  (Transformation|SetRelativeScale3D (Variables|Default|GetCuerpo) (Math|Vector|MakeVector (/ (- 82.0 _returnvalue_2) 82.0) 1.0 1.0))
  (if (> _returnvalue_2 0.0)
    (CallFunction|IncrementarTimer)
    (else
      (Transformation|SetRelativeLocation (Variables|Default|GetMitad%20Bola%201) "0.000000,0.0,141.000000" false false)
      (Transformation|SetRelativeLocation (Variables|Default|GetMitad%20Bola%202) "0.000000,0.0,141.000000" false false)
      (Transformation|SetRelativeScale3D (Variables|Default|GetCuerpo) "1.000000,1.000000,1.000000")
      (CallFunction|BorrarTimer))))