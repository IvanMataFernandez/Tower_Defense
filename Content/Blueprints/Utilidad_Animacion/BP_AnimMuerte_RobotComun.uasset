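; Death animation utility for the common robot that tips it over procedurally and plays a death sound.
; Inicializar stores the BaseRobot component to rotate.
; AnimarMuerte plays Muerte_Robot behind a first-frame check, then lowers relative roll at a delta-time-scaled rate, zeroing pitch and yaw.
; It increments a timer during the fall, then clamps at the final tilt and clears the timer.
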(event EventBeginPlay
  (|CallParentFunction) ; This node is disabled and will not be called.\nDrag off pins to build functionality.
)

(event EventTick
  (params (DeltaSeconds :type Float%20%28single-precision%29))
  (|CallParentFunction DeltaSeconds) ; This node is disabled and will not be called.\nDrag off pins to build functionality.
)

(fn Inicializar
  (params (Base%20Robot :type Scene%20Component%20Object%20Reference))
  (Variables|Default|SetBase%20Robot Base%20Robot))

(fn AnimarMuerte
  (bind _deltatime (Variables|Default|GetDeltaTime))
  (bind _base_robot (Variables|Default|GetBase%20Robot))
  (bind _returnvalue (* _deltatime -1e+02))
  (bind _relativerotation (Variables|/Script/Engine.SceneComponent|GetRelativeRotation _base_robot))
  (bind _returnvalue_2 (+ (.roll _relativerotation) _returnvalue))
  (if (.No%20ha%20pasado (CallFunction|ComprobarFrame 1))
    (CallFunction|SonarAudio "/Game/Blueprints/Audio/SFX/Muerte_Robot.Muerte_Robot"))
  (if (> _returnvalue_2 -7e+01)
    (Transformation|SetRelativeRotation (Variables|Default|GetBase%20Robot) (Math|Rotator|MakeRotator _returnvalue_2 0.0 0.0) false false)
    (CallFunction|IncrementarTimer)
    (else
      (Transformation|SetRelativeRotation (Variables|Default|GetBase%20Robot) "0.0,0.0,-70.000000" false false)
      (CallFunction|BorrarTimer))))