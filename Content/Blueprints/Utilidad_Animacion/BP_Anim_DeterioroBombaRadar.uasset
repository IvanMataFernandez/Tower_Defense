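; BP_Anim_DeterioroBombaRadar is an animation utility that shows a BombaRadar deteriorating through its three propellers (hélices).
; Inicializar stores the three propeller references and resets a flag tracking whether the first is destroyed.
; The first Deteriorar call hides propeller 1 and halves the speed of the other two.
; Later calls hide propeller 2 and halve propeller 3's speed again, so propeller 3 is never hidden here.
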(event EventBeginPlay
  (|CallParentFunction) ; This node is disabled and will not be called.\nDrag off pins to build functionality.
)

(event EventTick
  (params (DeltaSeconds :type Float%20%28single-precision%29)))

(fn Inicializar
  (params (Helice1 :type BP%20Anim%20Rotar%20Componente%20Object%20Reference) (Helice2 :type BP%20Anim%20Rotar%20Componente%20Object%20Reference) (Helice3 :type BP%20Anim%20Rotar%20Componente%20Object%20Reference))
  (Variables|Default|SetHelice1 Helice1)
  (Variables|Default|SetHelice2 Helice2)
  (Variables|Default|SetHelice3 Helice3)
  (Variables|Default|SetHelice1YaDestruida false))

(fn Deteriorar
  (bind _helice2 (Variables|Default|GetHelice2))
  (if (Variables|Default|GetHelice1YaDestruida)
    (Default|OcultarComponente _helice2)
    (else
      (Default|OcultarComponente (Variables|Default|GetHelice1))
      (Default|BajarVelocidadAMitad _helice2)
      (Variables|Default|SetHelice1YaDestruida true)))
  (Default|BajarVelocidadAMitad (Variables|Default|GetHelice3)))