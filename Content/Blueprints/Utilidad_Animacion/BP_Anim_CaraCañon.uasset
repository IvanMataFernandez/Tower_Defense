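; Animation utility for a cannon face ("CaraCañon") component that handles aiming, un-aiming and firing recoil.
; Inicializar stores the component, resets the recoil direction and sets up audio.
; Disparo plays the shot sound behind a frame check, then slides the component quickly back along local Y and more slowly home.
; Apuntar and Desapuntar rotate its roll between raised and level limits, using delta-time steps and clearing the timer on completion.
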(fn Disparo
  (bind _cara (Variables|Default|GetCara))
  (if (.No%20ha%20pasado (CallFunction|ComprobarFrame 1))
    (CallFunction|SonarAudio "/Game/Blueprints/Audio/SFX/Disparo_Cañon.Disparo_Cañon"))
  (if (Variables|Default|GetMoverHaciaAtras)
    ;[1 1 1] Animar cañón hacia atrás
    (Transformation|AddLocalOffset (Variables|Default|GetCara) (Math|Vector|MakeVector 0.0 (* (CallFunction|ObtenerDeltaTime) -7.5e+02) 0.0) false false)
    (if (<= (.y (Variables|/Script/Engine.SceneComponent|GetRelativeLocation (Variables|Default|GetCara))) -127.0)
      (Variables|Default|SetMoverHaciaAtras false))
    (CallFunction|IncrementarTimer :!label _label)
    (else
      ;[1 1 1] Animar cañón hacia adelante
      (Transformation|AddLocalOffset (Variables|Default|GetCara) (Math|Vector|MakeVector 0.0 (* (CallFunction|ObtenerDeltaTime) 2.5e+02) 0.0) false false)
      (if (>= (.y (Variables|/Script/Engine.SceneComponent|GetRelativeLocation _cara)) 0.0)
        (Transformation|SetRelativeLocation _cara "0, 0, 0" false false)
        (Variables|Default|SetMoverHaciaAtras true)
        (CallFunction|BorrarTimer)
        (else
          (goto _label))))))

(fn Inicializar
  (params (Componente :type Static%20Mesh%20Component%20Object%20Reference))
  (Variables|Default|SetCara Componente)
  (Variables|Default|SetMoverHaciaAtras true)
  (CallFunction|IncializarAudio))

(fn Apuntar
  (bind _deltatime (CallFunction|ObtenerDeltaTime))
  (bind _cara (Variables|Default|GetCara))
  (bind _returnvalue (* _deltatime 3e+02))
  (bind _relativerotation (Variables|/Script/Engine.SceneComponent|GetRelativeRotation _cara))
  (bind _returnvalue_2 (- (.roll _relativerotation) _returnvalue))
  (if (<= _returnvalue_2 0.0)
    (Transformation|SetRelativeRotation (Variables|Default|GetCara) "0, 0, 0" false false)
    (CallFunction|BorrarTimer)
    (else
      (Transformation|SetRelativeRotation (Variables|Default|GetCara) (Math|Rotator|MakeRotator _returnvalue_2 0.0 0.0) false false))))

(fn Desapuntar
  (bind _deltatime (CallFunction|ObtenerDeltaTime))
  (bind _cara (Variables|Default|GetCara))
  (bind _returnvalue (* _deltatime 9e+01))
  (bind _relativerotation (Variables|/Script/Engine.SceneComponent|GetRelativeRotation _cara))
  (bind _returnvalue_2 (+ (.roll _relativerotation) _returnvalue))
  (if (>= _returnvalue_2 3e+01)
    (Transformation|SetRelativeRotation (Variables|Default|GetCara) "0.0,0.0,30.000000" false false)
    (CallFunction|BorrarTimer)
    (else
      (Transformation|SetRelativeRotation (Variables|Default|GetCara) (Math|Rotator|MakeRotator _returnvalue_2 0.0 0.0) false false)
      (CallFunction|IncrementarTimer))))