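; Death-animation utility for the double cannon (CañonDoble) that tilts two face components apart.
; Inicializar stores the two faces, Cara1 and Cara2.
; AnimarMuerte rolls them in opposite directions at a frame-rate-scaled speed, using Cara2's roll as the reference, and calls IncrementarTimer on each step.
; Once the roll limit is reached, it snaps both to mirrored final angles and calls BorrarTimer.
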(event EventBeginPlay
  (|CallParentFunction) ; This node is disabled and will not be called.\nDrag off pins to build functionality.
)

(event EventTick
  (params (DeltaSeconds :type Float%20%28single-precision%29))
  (|CallParentFunction DeltaSeconds) ; This node is disabled and will not be called.\nDrag off pins to build functionality.
)

(fn Inicializar
  (params (Cara1 :type Static%20Mesh%20Component%20Object%20Reference) (Cara2 :type Static%20Mesh%20Component%20Object%20Reference))
  (Variables|Default|SetCara1 Cara1)
  (Variables|Components|SetCara2 Cara2))

(fn AnimarMuerte
  (bind _deltatime (Variables|Default|GetDeltaTime))
  (bind _cara2 (Variables|Components|GetCara2))
  (bind _returnvalue (* 6e+01 _deltatime))
  (bind _relativerotation (Variables|/Script/Engine.SceneComponent|GetRelativeRotation _cara2))
  (bind _returnvalue_2 (+ (.roll _relativerotation) _returnvalue))
  (if (>= _returnvalue_2 45.0)
    (Transformation|SetRelativeRotation _cara2 "0, 0,-45.000000" false false)
    (Transformation|SetRelativeRotation (Variables|Components|GetCara2) "0, 0,45.000000" false false)
    (CallFunction|BorrarTimer)
    (else
      (Transformation|SetRelativeRotation (Variables|Components|GetCara2) (Math|Rotator|MakeRotator _returnvalue_2 0.0 0.0) false false)
      (bind _result (Math|Float|NegateFloat _returnvalue_2)
        (:%20%20
          (Transformation|SetRelativeRotation (Variables|Default|GetCara1) (Math|Rotator|MakeRotator _result 0.0 0.0) false false)
          (CallFunction|IncrementarTimer))))))