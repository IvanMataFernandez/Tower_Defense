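; Animation utility Blueprint that spins three propellers (hélices) around their local yaw axis.
; Inicializar stores the three propeller references passed in by the caller.
; RotarHelice applies the same yaw step, DeltaTime scaled to one turn per second, to each via AddLocalRotation.
; Its own BeginPlay and Tick are disabled and DeltaTime is not assigned here, so the rotation does not drive itself.
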(event EventBeginPlay
  (|CallParentFunction) ; This node is disabled and will not be called.\nDrag off pins to build functionality.
)

(event EventTick
  (params (DeltaSeconds :type Float%20%28single-precision%29))
  (|CallParentFunction DeltaSeconds) ; This node is disabled and will not be called.\nDrag off pins to build functionality.
)

(fn Inicializar
  (params (Helice%201 :type Static%20Mesh%20Component%20Object%20Reference) (Helice%202 :type Static%20Mesh%20Component%20Object%20Reference) (Helice%203 :type Static%20Mesh%20Component%20Object%20Reference))
  (Variables|Default|SetHelice%201 Helice%201)
  (Variables|Default|SetHelice%202 Helice%202)
  (Variables|Default|SetHelice%203 Helice%203))

(fn RotarHelice
  (LocalVariables|SetRotacion (* (Variables|Default|GetDeltaTime) 3.6e+02))
  (Transformation|AddLocalRotation (Variables|Default|GetHelice%201) (Math|Rotator|MakeRotator 0.0 0.0 (LocalVariables|GetRotacion)) false false)
  (Transformation|AddLocalRotation (Variables|Default|GetHelice%202) (Math|Rotator|MakeRotator 0.0 0.0 (LocalVariables|GetRotacion)) false false)
  (Transformation|AddLocalRotation (Variables|Default|GetHelice%203) (Math|Rotator|MakeRotator 0.0 0.0 (LocalVariables|GetRotacion)) false false))