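; In-match GameMode for a tower-and-wave game that drives the UI flow from tower selection through countdown, gameplay and victory or defeat, plus pause.
; Each event has BP_MandoDeJugador_EnPartida create or remove indexed HUDs, then initializes the cast widget.
; Tower picks and reward clicks are forwarded to FinSeleccionTorres and ProcesarClickEnRecompensa, defined outside this graph.
; BeginPlay also sets overall scalability to the lowest level.
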(event Custom|Click%20En%20Recompensa
  (Class|MandoDeJugadorEnPartida|QuitarHUD (Variables|Default|GetMandoDeJugador))
  (Class|GameModeEnPartida|ProcesarClickEnRecompensa))

(event Custom|Fin%20De%20Seleccion%20Torres
  (params (IDsTorresElegidas :type Array%20of%20Integers))
  (Class|MandoDeJugadorEnPartida|QuitarHUD (Variables|Default|GetMandoDeJugador))
  (Class|GameModeEnPartida|FinSeleccionTorres IDsTorresElegidas))

(event Custom|Pausar
  (Game|SetGamePaused true)
  (bind _returnvalue (Class|MandoDeJugadorEnPartida|CrearHUD (Variables|Default|GetMandoDeJugador) 5))
  (bind _asbp_menu_de_pausa (Utilities|Casting|CastToBP_MenuDePausa _returnvalue))
  (Default|IniciarUI _asbp_menu_de_pausa))

(event Custom|Despausar
  (bind _mandodejugador (Variables|Default|GetMandoDeJugador))
  (bind _returnvalue (Class|MandoDeJugadorEnPartida|ObtenerHUD _mandodejugador))
  (Class|MandoDeJugadorEnPartida|QuitarUltimaHUDAnadida _mandodejugador)
  (Game|SetGamePaused false)
  (bind _asbp_interfaz_en_partida (Utilities|Casting|CastToBP_InterfazEnPartida _returnvalue)
    (:then
      (Default|Despausar _asbp_interfaz_en_partida))
    (:CastFailed
      (bind _asbp_interfaz_seleccion (Utilities|Casting|CastToBP_InterfazSeleccion _returnvalue))
      (Default|Despausar _asbp_interfaz_seleccion))))

(event EventBeginPlay
  (bind _returnvalue (Settings|GetGameUserSettings))
  (Class|GameUserSettings|SetOverallScalabilityLevel _returnvalue))

(event EventCrearInterfazDeDerrota
  (bind _returnvalue (Class|MandoDeJugadorEnPartida|CrearHUD (Variables|Default|GetMandoDeJugador) 3))
  (bind _asbp_interfaz_derrota (Utilities|Casting|CastToBP_InterfazDerrota _returnvalue))
  (Default|IniciarUI _asbp_interfaz_derrota))

(event EventCrearInterfazDeCuentaAtras
  (bind _returnvalue (Class|MandoDeJugadorEnPartida|CrearHUD (Variables|Default|GetMandoDeJugador) 1))
  (bind _asbp_interfaz_cuenta_atras (Utilities|Casting|CastToBP_InterfazCuentaAtras _returnvalue))
  (Default|IniciarUI _asbp_interfaz_cuenta_atras))

(event EventCrearInterfazDePartida
  (bind _mandodejugador (Variables|Default|GetMandoDeJugador))
  (Class|MandoDeJugadorEnPartida|QuitarHUD (Variables|Default|GetMandoDeJugador))
  (bind _returnvalue (Class|MandoDeJugadorEnPartida|CrearHUD _mandodejugador 2))
  (bind _asbp_interfaz_en_partida (Utilities|Casting|CastToBP_InterfazEnPartida _returnvalue))
  (bind _output_get (Variables|Default|SetInterfazEnPartida _asbp_interfaz_en_partida))
  (Default|IniciarUI _output_get (Variables|Default|GetGrandesOleadas) (Class|MandoDeJugadorEnPartida|GetTorresElegidas _mandodejugador)))

(event EventCrearInterfazSeleccionDeTorres
  (bind _asbp_mando_de_jugador_en_partida (Utilities|Casting|CastToBP_MandoDeJugador_EnPartida (Game|GetPlayerController 0)))
  (bind _output_get (Variables|Default|SetMandoDeJugador _asbp_mando_de_jugador_en_partida))
  (bind _returnvalue (Class|MandoDeJugadorEnPartida|CrearHUD _output_get))
  (bind _asbp_interfaz_seleccion (Utilities|Casting|CastToBP_InterfazSeleccion _returnvalue))
  (Default|IniciarUI _asbp_interfaz_seleccion))

(event EventQuitarInterfaz
  (Class|MandoDeJugadorEnPartida|QuitarHUD (Variables|Default|GetMandoDeJugador)))

(event EventComunicarVictoria
  (params (Nivel :type Integer) (PosXDrop :type Float%20%28single-precision%29) (PosYDrop :type Float%20%28single-precision%29))
  (bind _mandodejugador (Variables|Default|GetMandoDeJugador))
  (bind _asbp_interfaz_en_partida (Utilities|Casting|CastToBP_InterfazEnPartida (Class|MandoDeJugadorEnPartida|ObtenerHUD _mandodejugador)))
  (Default|BloquearBotones _asbp_interfaz_en_partida)
  (bind _returnvalue (Class|MandoDeJugadorEnPartida|CrearHUD _mandodejugador 4))
  (bind _asbp_interfaz_victoria (Utilities|Casting|CastToBP_InterfazVictoria _returnvalue))
  (Default|IniciarUI _asbp_interfaz_victoria Nivel PosXDrop PosYDrop))

(event EventComunicarAvanceOleadaUI
  (Default|AvanzarBarra (Variables|Default|GetInterfazEnPartida)))

(fn ConstructionScript)