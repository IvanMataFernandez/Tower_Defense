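; BP_PlayerPawn_EnPartida is the in-match player pawn, providing a timed camera pitch rotation to a target angle.
; RotarCamEnPitchA derives a constant per-step pitch increment from the target and duration, then starts a looping timer at the DeltaTiempo interval.
; Each RotarCam tick adds that increment to the camera's relative pitch, forcing roll and yaw to zero, and clears the timer once the duration has elapsed.
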(event Custom|Rotar%20Cam
  (Transformation|SetRelativeRotation (Variables|Default|GetCamara) (Math|Rotator|MakeRotator 0.0 (+ (.pitch (Variables|/Script/Engine.SceneComponent|GetRelativeRotation (Variables|Default|GetCamara))) (Variables|Default|GetVelocidad%20Pitch)) 0.0) false false)
  (Variables|Default|SetMomento%20Actual (+ (Variables|Default|GetMomento%20Actual) (Variables|Default|GetDeltaTiempo)))
  (if (>= (Variables|Default|GetMomento%20Actual) (Variables|Default|GetTiempo%20Target))
    (Utilities|Time|ClearandInvalidateTimerbyHandle (Variables|Default|GetTimerHandle))))

(event EventRotarCamEnPitchA
  (params (Pitch :type Float%20%28single-precision%29) (Duracion :type Float%20%28single-precision%29))
  (Variables|Default|SetMomento%20Actual 0.0)
  (Variables|Default|SetTiempo%20Target Duracion)
  (Variables|Default|SetVelocidad%20Pitch (* (/ (- Pitch (.pitch (Variables|/Script/Engine.SceneComponent|GetRelativeRotation (Variables|Default|GetCamara)))) (Variables|Default|GetTiempo%20Target)) (Variables|Default|GetDeltaTiempo)))
  (bind _returnvalue (Utilities|Time|SetTimerbyEvent (delegate Custom|Rotar%20Cam) (Variables|Default|GetDeltaTiempo) true))
  (Variables|Default|SetTimerHandle _returnvalue))

(fn ConstructionScript)