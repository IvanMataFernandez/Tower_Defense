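; Menu game mode that boots the main menu and switches between main menu, tutorial and settings screens.
; On BeginPlay it loads the current level from the BP_Guardador save slot, or creates a new save with starting unlocked towers and default video settings, then loads user settings.
; Each switch event asks BP_MandoDeJugador_EnMenu to change interface by index, then initializes the returned widget, passing the level to the main menu.
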(event Custom|Cambiar%20A%20Ajustes
  (bind _asbp_mando_de_jugador_en_menu (Utilities|Casting|CastToBP_MandoDeJugador_EnMenu (Game|GetPlayerController 0)))
  (bind _returnvalue (Class|MandoDeJugadorEnMenu|CambiarAInterfaz _asbp_mando_de_jugador_en_menu 2))
  (bind _asbp_menu_de_ajustes (Utilities|Casting|CastToBP_MenuDeAjustes _returnvalue))
  (Default|IniciarUI _asbp_menu_de_ajustes))

(event Custom|Cambiar%20A%20MenuPrincipal
  (bind _asbp_mando_de_jugador_en_menu (Utilities|Casting|CastToBP_MandoDeJugador_EnMenu (Game|GetPlayerController 0)))
  (bind _returnvalue (Class|MandoDeJugadorEnMenu|CambiarAInterfaz _asbp_mando_de_jugador_en_menu))
  (bind _asbp_interfaz_menu_principal (Utilities|Casting|CastToBP_InterfazMenuPrincipal _returnvalue))
  (Default|IniciarUI _asbp_interfaz_menu_principal (Variables|Default|GetNivelAct)))

(event Custom|Cambiar%20A%20Tutorial
  (bind _asbp_mando_de_jugador_en_menu (Utilities|Casting|CastToBP_MandoDeJugador_EnMenu (Game|GetPlayerController 0)))
  (bind _returnvalue (Class|MandoDeJugadorEnMenu|CambiarAInterfaz _asbp_mando_de_jugador_en_menu 1))
  (bind _asbp_interfaz_tutorial (Utilities|Casting|CastToBP_InterfazTutorial _returnvalue))
  (Default|IniciarUI _asbp_interfaz_tutorial))

(event EventBeginPlay
  (bind _returnvalue (Settings|GetGameUserSettings))
  (bind _returnvalue_2 (SaveGame|DoesSaveGameExist "save"))
  (if _returnvalue_2
    (bind _returnvalue_3 (SaveGame|LoadGamefromSlot "save"))
    (bind _asbp_guardador (Utilities|Casting|CastToBP_Guardador _returnvalue_3))
    (Variables|Default|SetNivelAct (Variables|/Script/Tower_Defense.Guardador|GetNivel _asbp_guardador))
    (else
      (CallFunction|CrearNuevaSave)
      (Variables|Default|SetNivelAct 1)
      (Class|GameUserSettings|SetFullscreenMode _returnvalue "Fullscreen")
      (Class|GameUserSettings|SetFrameRateLimit _returnvalue 0.0)
      (Class|GameUserSettings|SetVSyncEnabled _returnvalue true)
      (Class|GameUserSettings|ApplySettings _returnvalue true)))
  (Class|GameUserSettings|LoadSettings _returnvalue false)
  (CallFunction|CambiarAMenuPrincipal))

(fn ConstructionScript)

(fn CrearNuevaSave
  (bind _returnvalue (SaveGame|CreateSaveGameObject "/Game/Blueprints/Jugador_Y_Gamemode/BP_Guardador.BP_Guardador_C"))
  (Variables|/Script/Tower_Defense.Guardador|SetNivel _returnvalue 1)
  (Utilities|Array|Add (Variables|/Script/Tower_Defense.Guardador|GetIDsTorresDesbloqueadas _returnvalue) 8)
  (Utilities|Array|Add (Variables|/Script/Tower_Defense.Guardador|GetIDsTorresDesbloqueadas _returnvalue) 0)
  (Variables|/Script/Tower_Defense.Guardador|SetIDsTorresDesbloqueadas _returnvalue (Variables|/Script/Tower_Defense.Guardador|GetIDsTorresDesbloqueadas _returnvalue))
  (SaveGame|SaveGametoSlot _returnvalue "save"))