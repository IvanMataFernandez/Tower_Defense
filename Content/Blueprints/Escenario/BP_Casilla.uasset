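; BP_Casilla is a board tile on which towers are placed, including cannons, lasers, solar panels, mines, bombs and shields.
; SpawnearTorre maps an ID to a tower class through ElegirTorre, spawns it slightly above the tile and passes it to PonerTorre.
; DestacarCasilla only stores the highlight flag, which PonerMaterialBase clears.
; Placement and destruction events share one audio component with swapped sounds, and destruction adds an explosion emitter.
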(event EventBeginPlay
  (Variables|Default|SetCasillaEncendida false))

(event EventAnimarPonerTorre
  (bind _componentedeaudio (Variables|Default|GetComponenteDeAudio))
  (Audio|Components|Audio|SetSound _componentedeaudio "/Game/Blueprints/Audio/SFX/Colocar_Torre.Colocar_Torre")
  (Audio|Components|Audio|Play _componentedeaudio 0.0))

(event EventPonerMaterialBase
  (if (Variables|Default|GetCasillaEncendida)
    (CallFunction|DestacarCasilla false)))

(event EventSpawnearTorre
  (params (ID :type Byte :default 0))
  (bind _returnvalue (Transformation|GetActorLocation))
  (bind _clase (CallFunction|ElegirTorre (Math|Conversions|ToInteger(Byte) ID)))
  (bind _returnvalue_2 (Game|SpawnActorfromClass _clase (Math|Transform|MakeTransform (Math|Vector|MakeVector (.x _returnvalue) (.y _returnvalue) (+ (.z _returnvalue) 25.6)) "0, 0, 0" "1.000000,1.000000,1.000000") "AlwaysSpawn" 0 0))
  (bind _astorre (Utilities|Casting|CastToTorre _returnvalue_2))
  (Class|Casilla|PonerTorre _astorre))

(event EventAnimarDestruirTorre
  (bind _componentedeaudio (Variables|Default|GetComponenteDeAudio))
  (Audio|Components|Audio|SetSound _componentedeaudio "/Game/Blueprints/Audio/SFX/Quitar_Torre.Quitar_Torre")
  (Effects|SpawnEmitterAttached "/Game/Realistic_Starter_VFX_Pack_Vol2/Particles/Explosion/P_Explosion_Big_B.P_Explosion_Big_B" (Variables|Character|GetMesh) "None")
  (Audio|Components|Audio|Play _componentedeaudio 0.0))

(fn ConstructionScript)

(fn ElegirTorre
  (params (Seleccion :type Integer))
  (switch int Seleccion
    (:0
      (return "/Game/Blueprints/Entidades/Torres/BP_Cañon.BP_Cañon_C"))
    (:1
      (return "/Game/Blueprints/Entidades/Torres/BP_CañonDoble.BP_CañonDoble_C"))
    (:2
      (return "/Game/Blueprints/Entidades/Torres/BP_PistolaLaser.BP_PistolaLaser_C"))
    (:8
      (return "/Game/Blueprints/Entidades/Torres/BP_PanelSolar.BP_PanelSolar_C"))
    (:9
      (return "/Game/Blueprints/Entidades/Torres/BP_PanelSolarDoble.BP_PanelSolarDoble_C"))
    (:11
      (return "/Game/Blueprints/Entidades/Torres/BP_Mina.BP_Mina_C"))
    (:12
      (return "/Game/Blueprints/Entidades/Torres/BP_Bomba.BP_Bomba_C"))
    (:16
      (return "/Game/Blueprints/Entidades/Torres/BP_Escudo.BP_Escudo_C"))))

(fn DestacarCasilla
  (params (Destacar :type Boolean))
  (Variables|Default|SetCasillaEncendida Destacar)
  (return))