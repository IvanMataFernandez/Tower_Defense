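; BP_Casilla2 is a board tile that spawns a tower or structure on itself when its SpawnearTorre event is called.
; The event switches on the received ID to pick a class among cannons, a laser pistol, solar panels and a bomb.
; All handled IDs share one spawn step that places the actor slightly above the tile's location and stores it in Torre.
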(event EventSpawnearTorre
  (params (ID :type Byte :default 0))
  (bind _returnvalue (Transformation|GetActorLocation))
  ;[1 1 1] Elegir tipo de torre para spawnear
  (switch int (Math|Conversions|ToInteger(Byte) ID)
    (:0
      (Variables|Default|SetTorreSpawned "/Game/Blueprints/Entidades/Torres/BP_Cañon.BP_Cañon_C"))
    (:1
      (Variables|Default|SetTorreSpawned "/Game/Blueprints/Entidades/Torres/BP_CañonDoble.BP_CañonDoble_C"))
    (:2
      (Variables|Default|SetTorreSpawned "/Game/Blueprints/Entidades/Torres/BP_PistolaLaser.BP_PistolaLaser_C"))
    (:8
      (Variables|Default|SetTorreSpawned "/Game/Blueprints/Entidades/Torres/BP_PanelSolar.BP_PanelSolar_C"))
    (:9
      (Variables|Default|SetTorreSpawned "/Game/Blueprints/Entidades/Torres/BP_PanelSolarDoble.BP_PanelSolarDoble_C"))
    (:11
      (Variables|Default|SetTorreSpawned "/Game/Blueprints/Entidades/Torres/BP_Bomba.BP_Bomba_C")))
  (bind _returnvalue_2 (Game|SpawnActorfromClass (Variables|Default|GetTorreSpawned) (Math|Transform|MakeTransform (Math|Vector|MakeVector (.x _returnvalue) (.y _returnvalue) (+ (.z _returnvalue) 1e+02)) "0, 0, 0" "1.000000,1.000000,1.000000") "Undefined" 0 0))
  (Variables|Default|SetTorre _returnvalue_2))

(fn ConstructionScript)