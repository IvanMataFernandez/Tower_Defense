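; BP_ZonaSpawnRobotEnPartida is a spawner that materializes robot enemies or units during a match.
; Its MaterealizarRobot event receives an ID and a position, then spawns the matching robot there, always spawning regardless of collision.
; The ElegirRobot function maps the numeric ID to a robot class, covering simple, leader, medium, tough, bomb, radar bomb and concealer variants, with a gap in the ID range.
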(event EventMaterealizarRobot
  (params (ID :type Integer) (Posicion :type Vector :default "0, 0, 0"))
  (Game|SpawnActorfromClass (CallFunction|ElegirRobot ID) (Math|Transform|MakeTransform Posicion "0, 0, 0" "1.000000,1.000000,1.000000") "AlwaysSpawn" 0 0))

(fn ConstructionScript)

(fn ElegirRobot
  (params (ID :type Integer))
  (switch int ID
    (:0
      (return "/Game/Blueprints/Entidades/Robots/BP_RobotSimple.BP_RobotSimple_C"))
    (:1
      (return "/Game/Blueprints/Entidades/Robots/BP_RobotLider.BP_RobotLider_C"))
    (:2
      (return "/Game/Blueprints/Entidades/Robots/BP_RobotMedio.BP_RobotMedio_C"))
    (:3
      (return "/Game/Blueprints/Entidades/Robots/BP_RobotDuro.BP_RobotDuro_C"))
    (:8
      (return "/Game/Blueprints/Entidades/Robots/BP_RobotBomba.BP_RobotBomba_C"))
    (:9
      (return "/Game/Blueprints/Entidades/Robots/BP_RobotBombaRadar.BP_RobotBombaRadar_C"))
    (:10
      (return "/Game/Blueprints/Entidades/Robots/BP_RobotOcultador.BP_RobotOcultador_C"))))