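; BP_ZonaSpawnRobot is a spawn zone that creates robot actors in a chosen row when its SpawnearRobot event is called.
; The row indexes an array of X offsets from the zone's location, and the box extent drops the spawn height to the zone's bottom, ignoring collisions.
; ElegirRobot maps basic, bomb and radar-bomb robot classes, but its selector is fixed at 0 rather than the passed ID.
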(event EventSpawnearRobot
  (params (ID :type Integer) (Fila :type Integer))
  (bind _returnvalue (Transformation|GetActorLocation))
  (bind _newparam (CallFunction|ElegirRobot ID))
  (Game|SpawnActorfromClass _newparam (Math|Transform|MakeTransform (Math|Vector|MakeVector (+ (Utilities|Array|Get(acopy) (Variables|Default|GetPosicionesDeSpawn) Fila) (.x _returnvalue)) (.y _returnvalue) (- (.z _returnvalue) (.z (Components|Box|GetScaledBoxExtent (Variables|Default|GetZonaDeSpawn))))) "0, 0, 0" "1.000000,1.000000,1.000000") "AlwaysSpawn" 0 0))

(fn ConstructionScript)

(fn ElegirRobot
  (params (ID :type Integer))
  (switch int 0
    (:0
      (return "/Game/Blueprints/Entidades/Robots/BP_RobotBásico.BP_RobotBásico_C"))
    (:8
      (return "/Game/Blueprints/Entidades/Robots/BP_RobotBomba.BP_RobotBomba_C"))
    (:9
      (return "/Game/Blueprints/Entidades/Robots/BP_RobotBombaRadar.BP_RobotBombaRadar_C"))))