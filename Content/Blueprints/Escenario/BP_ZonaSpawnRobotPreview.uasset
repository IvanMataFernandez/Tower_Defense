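; Spawn zone that places robot actors, likely for previewing them, in a grid inside the ZonaDeSpawn box.
; EventoSpawnearRobot takes an ID and an index, using ElegirRobot to map the ID to a robot Blueprint class.
; The index sets the grid cell through division and modulo by three, starting from the box's bottom at its minimum-Y side.
; Robots always spawn regardless of collision, with a fixed rotation.
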(event EventEventoSpawnearRobot
  (params (ID :type Integer) (Numero :type Integer))
  (bind _returnvalue (Transformation|GetActorLocation))
  (bind _zonadespawn (Variables|Default|GetZonaDeSpawn))
  (bind _returnvalue_2 (Components|Box|GetScaledBoxExtent _zonadespawn))
  (Game|SpawnActorfromClass (CallFunction|ElegirRobot ID) (Math|Transform|MakeTransform (Math|Vector|MakeVector (+ (* (/ Numero 3) 400) (.x _returnvalue)) (+ (* (Math|Integer|%(Integer) Numero 3) 400) (- (.y _returnvalue) (.y _returnvalue_2))) (- (.z _returnvalue) (.z _returnvalue_2))) "0.000000,-90.000000, 0" "1.000000,1.000000,1.000000") "AlwaysSpawn" 0 0))

(fn ConstructionScript)

(fn ElegirRobot
  (params (ID :type Integer))
  (switch int ID
    (:0
      (return "/Game/Blueprints/Entidades/Robots/BP_RobotBásico.BP_RobotBásico_C"))
    (:1
      (return "/Game/Blueprints/Entidades/Robots/BP_RobotLider.BP_RobotLider_C"))
    (:2
      (return "/Game/Blueprints/Entidades/Robots/BP_RobotMedio.BP_RobotMedio_C"))
    (:3
      (return "/Game/Blueprints/Entidades/Robots/BP_RobotDuro.BP_RobotDuro_C"))
    (:8
      (return "/Game/Blueprints/Entidades/Robots/BP_RobotBomba.BP_RobotBomba_C"))
    (:9
      (return "/Game/Blueprints/Entidades/Robots/BP_RobotBombaRadar.BP_RobotBombaRadar_C"))
    (:10
      (return "/Game/Blueprints/Entidades/Robots/BP_RobotOcultador.BP_RobotOcultador_C"))))